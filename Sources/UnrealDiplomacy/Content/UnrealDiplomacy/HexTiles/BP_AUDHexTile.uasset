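; Hex tile actor for UnrealDiplomacy that handles clicking, selection highlighting and visual refresh.
; Clicks on WORLD-type tiles are forwarded to the UD player controller, and selection events swap the Border material between selected and unselected.
; RefreshVisuals flips the VisualChangeTag boolean, whose OnRep calls VisualUpdate on replication, an empty function in this Blueprint.
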(event Custom|OnSelected
  (Rendering|Material|SetMaterial (Variables|Default|GetBorder) 0 "/Game/UnrealDiplomacy/HexTiles/MI_HexTile_BackgroundSelected.MI_HexTile_BackgroundSelected"))

(event Custom|OnDeselected
  (Rendering|Material|SetMaterial (Variables|Default|GetBorder) 0 "/Game/UnrealDiplomacy/HexTiles/MI_HexTile_BackgroundUnselected.MI_HexTile_BackgroundUnselected"))

(event Custom|RefreshVisuals
  (Utilities|UpdateVisualChangeTag))

(event EventBeginPlay)

(event MouseInput|EventActorOnClicked
  (params (ButtonPressed :type Key%20Structure :default "None"))
  (switch Utilities|FlowControl|Switch|SwitchonEHexTileType (Variables|Default|GetTileType)
    (:WORLD
      (bind _asbp_udplayer_controller (CallFunction|GetUDPlayerController))
      (Default|OnTileClicked _asbp_udplayer_controller self))))

(fn ConstructionScript)

(fn OnRepVisualChangeTag
  (CallFunction|VisualUpdate)
  (return))

(fn VisualUpdate
  (return))