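; Skirmish match HUD that creates the lobby and in-game widgets up front and switches between them by match state.
; Each widget or shared view model is bound to the action model as authority and refreshed on model updates, with nation list items built per player.
; Confirmed surrender and leave clicks go to the game instance, while lobby setting changes go straight to the server through the player controller.
; Tile and nation selection open their management panels.
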(event EventBeginPlay
  ;[1 1 1] Initialization
  (CallFunction|LogInfo "BP_UDSkirmishHUD: Begin Play." false))

(event Custom|InvokeOnLeaveGameClicked
  ;[1 1 1] All callbacks from Game UI elements are required to go through here, this is done by explicit confirmation from user
  (bind _asbp_uudgame_instance (CallFunction|GetUDGameInstance))
  (Default|LeaveGame _asbp_uudgame_instance))

(event Custom|InvokeOnHideClicked
  (params (Widget :type User%20Widget%20Object%20Reference))
  ;[1 1 1] All callbacks from Game UI elements are required to go through here, this is done by explicit confirmation from user
  (MatchUI|HideWidget Widget))

(event Custom|InvokeOnSurrenderGameClicked
  ;[1 1 1] All callbacks from Game UI elements are required to go through here, this is done by explicit confirmation from user
  (bind _asbp_uudgame_instance (CallFunction|GetUDGameInstance))
  (Default|SurrenderGame _asbp_uudgame_instance))

(event Custom|OnUpdateLobbySettings
  (params (Owner :type Integer) (LobbyData :type FUD%20Lobby%20Settings%20Structure) (IsOwner :type Boolean))
  ;[1 1 1] Updates based on data changed
  (MatchUIUpdates|UpdateLobbySettings Owner LobbyData IsOwner))

(event Custom|OnUpdateMatchStateUI
  (params (MatchUI :type EUDMatchState%20Enum :default "NewEnumerator0"))
  ;[1 1 1] Updates based on data changed
  (MatchUI|SwitchMatchUI MatchUI))

(event Custom|OnUpdateLobbyMembers
  (params (Members :type Array%20of%20FUD%20Player%20Data%20Structures))
  ;[1 1 1] Updates based on data changed
  (MatchUIUpdates|UpdateLobbyMembers Members))

(event Custom|OnUpdateLobbyPlayerSettings
  (params (NationSettings :type FUD%20Nation%20Settings%20Structure))
  ;[1 1 1] Updates based on data changed
  (MatchUIUpdates|UpdateLobbyPlayerSettings NationSettings))

(event Custom|OnChangedLobbySettings
  (params (NewSettings :type FUD%20Lobby%20Settings%20Structure))
  ;[1 1 1] Updates from user input that needs to be propagated to server, this contains automatic actions, no confirmation is done for these
  (bind _asbp_udplayer_controller (CallFunction|GetUDPlayerController))
  (Default|ServerUpdateLobbySettings _asbp_udplayer_controller NewSettings))

(event Custom|OnChangedLobbyPlayerSettings
  (params (NewNationSettings :type FUD%20Nation%20Settings%20Structure))
  ;[1 1 1] Updates from user input that needs to be propagated to server, this contains automatic actions, no confirmation is done for these
  (bind _asbp_udplayer_controller (CallFunction|GetUDPlayerController))
  (Default|ServerUpdateLobbyPlayerSettings _asbp_udplayer_controller NewNationSettings))

(event Custom|BindModels
  (params (ActionModel :type UD%20Action%20Administrator%20Object%20Reference))
  (bind _output_get (Variables|Default|SetAction%20Model ActionModel))
  (Utilities|FlowControl|Sequence
    (:then_0
      (Class|UDEndTurnViewModel|SetAuthority (Variables|/Game/UnrealDiplomacy/Skirmish/UI/WBP_TurnCounter.WBP_TurnCounter_C|GetUDEndTurnViewModel (Variables|Widget|GetTurnCounterWidget)) _output_get))
    (:then_1
      (Class|UDViewModelBase|SetAuthority (Variables|/Game/UnrealDiplomacy/Lobby/UI/WBP_Lobby.WBP_Lobby_C|GetUDLobbyViewModel (Variables|Widget|GetLobbyWidget)) _output_get))
    (:then_2
      (Class|UDViewModelBase|SetAuthority (Variables|/Game/UnrealDiplomacy/Skirmish/UI/WBP_TileManagement.WBP_TileManagement_C|GetUDTileOverviewViewModel (Variables|Widget|GetTileManegementWidget)) _output_get))
    (:then_3
      (Class|UDViewModelBase|SetAuthority (Variables|Default|GetGoldInformationViewModel) _output_get))
    (:then_4
      (Class|UDViewModelBase|SetAuthority (Variables|/Game/UnrealDiplomacy/Skirmish/UI/WBP_NationManagement.WBP_NationManagement_C|GetUDNationOverviewViewModel (Variables|Widget|GetNationManagementWidget)) _output_get))
    (:then_5
      (ViewModels|DefineNationItemViewModels))))

(event Custom|TileSelectionChanged
  (params (Position :type Int%20Point%20Structure))
  (MatchUIUpdates|UpdateTileManagement Position))

(event Custom|UpdateModels
  (Utilities|FlowControl|Sequence
    (:then_0
      (Class|UDEndTurnViewModel|OnUpdate (Variables|/Game/UnrealDiplomacy/Skirmish/UI/WBP_TurnCounter.WBP_TurnCounter_C|GetUDEndTurnViewModel (Variables|Widget|GetTurnCounterWidget))))
    (:then_1
      (Class|UDViewModelBase|OnUpdate (Variables|/Game/UnrealDiplomacy/Lobby/UI/WBP_Lobby.WBP_Lobby_C|GetUDLobbyViewModel (Variables|Widget|GetLobbyWidget))))
    (:then_2
      (Class|UDViewModelBase|OnUpdate (Variables|/Game/UnrealDiplomacy/Skirmish/UI/WBP_TileManagement.WBP_TileManagement_C|GetUDTileOverviewViewModel (Variables|Widget|GetTileManegementWidget))))
    (:then_3
      (Class|UDViewModelBase|OnUpdate (Variables|Default|GetGoldInformationViewModel)))
    (:then_4
      (Class|UDViewModelBase|OnUpdate (Variables|/Game/UnrealDiplomacy/Skirmish/UI/WBP_NationManagement.WBP_NationManagement_C|GetUDNationOverviewViewModel (Variables|Widget|GetNationManagementWidget))))
    (:then_5
      (ViewModels|OnUpdateNationItemViewModels))
    (:then_6
      (bind _returnvalue (Class|UDActionAdministrator|IsGameinProgress (Variables|Default|GetAction%20Model)))
      (if _returnvalue
        (MatchUI|SwitchMatchUI "NewEnumerator1")
        (else
          (MatchUI|SwitchMatchUI "NewEnumerator0"))))))

(event Custom|NationSelectionChanged
  (params (PlayerUniqueId :type Integer))
  (MatchUIUpdates|UpdateNationManagement))

(fn ConstructionScript
  ;[1 1 1] Create all UI elements in advance
  (Utilities|FlowControl|Sequence
    (:then_0
      (ViewModels|PrepareGlobalViewModels))
    (:then_1
      (Widgets|PrepareLobby))
    (:then_2
      (Widgets|PrepareNationInformationList))
    (:then_3
      (Widgets|PrepareTurnCounter))
    (:then_4
      (Widgets|PrepareTileManagement))
    (:then_5
      (Widgets|PreparePlayerInformationBar))
    (:then_6
      (Widgets|PrepareNationManagement))))

(fn PrepareLobby
  (Utilities|IsValid (Variables|Widget|GetLobbyWidget)
    (:Is%20Valid
      _)
    (:Is%20Not%20Valid
      (bind _returnvalue (UserInterface|CreateWidget "/Game/UnrealDiplomacy/Lobby/UI/WBP_Lobby.WBP_Lobby_C" (Game|GetPlayerController 0) 0))
      (bind _output_get (Variables|Widget|SetLobbyWidget _returnvalue))
      (bind _returnvalue_2 (Game|ConstructObjectfromClass _output_get "/Script/UnrealDiplomacy.UDLobbyViewModel"))
      (Default|SetUDLobbyViewModel _output_get _returnvalue_2)))
  (return (Variables|Widget|GetLobbyWidget)))

(fn PrepareTurnCounter
  (Utilities|IsValid (Variables|Widget|GetTurnCounterWidget)
    (:Is%20Valid
      _)
    (:Is%20Not%20Valid
      (bind _returnvalue (UserInterface|CreateWidget "/Game/UnrealDiplomacy/Skirmish/UI/WBP_TurnCounter.WBP_TurnCounter_C" (Game|GetPlayerController 0) 0))
      (bind _output_get (Variables|Widget|SetTurnCounterWidget _returnvalue))
      (bind _returnvalue_2 (Game|ConstructObjectfromClass _output_get "/Script/UnrealDiplomacy.UDEndTurnViewModel"))
      (Default|SetUDEndTurnViewModel _output_get _returnvalue_2)))
  (return (Variables|Widget|GetTurnCounterWidget)))

(fn PreparePlayerInformationBar
  (Utilities|IsValid (Variables|Widget|GetPlayerInformationBarWidget)
    (:Is%20Valid
      _)
    (:Is%20Not%20Valid
      (bind _returnvalue (UserInterface|CreateWidget "/Game/UnrealDiplomacy/Skirmish/UI/WBP_PlayerInformationBar.WBP_PlayerInformationBar_C" (Game|GetPlayerController 0)))
      (bind _output_get (Variables|Widget|SetPlayerInformationBarWidget _returnvalue))
      (Default|SetDisplayedResourceInfos _output_get (Variables|Default|GetGoldInformationViewModel))))
  (return (Variables|Widget|GetPlayerInformationBarWidget)))

(fn PrepareTileManagement
  (Utilities|IsValid (Variables|Widget|GetTileManegementWidget)
    (:Is%20Valid
      _)
    (:Is%20Not%20Valid
      (bind _returnvalue (UserInterface|CreateWidget "/Game/UnrealDiplomacy/Skirmish/UI/WBP_TileManagement.WBP_TileManagement_C" (Game|GetPlayerController 0) 0))
      (bind _output_get (Variables|Widget|SetTileManegementWidget _returnvalue))
      (bind _returnvalue_2 (Game|ConstructObjectfromClass _output_get "/Script/UnrealDiplomacy.UDTileOverviewViewModel"))
      (Default|SetUDTileOverviewViewModel _output_get _returnvalue_2)))
  (return (Variables|Widget|GetTileManegementWidget)))

(fn PrepareNationInformationList
  (Utilities|IsValid (Variables|Widget|GetNationInformationListWidget)
    (:Is%20Valid
      _)
    (:Is%20Not%20Valid
      (bind _returnvalue (UserInterface|CreateWidget "/Game/UnrealDiplomacy/Skirmish/UI/WBP_NationInformationList.WBP_NationInformationList_C" (Game|GetPlayerController 0)))
      (Variables|Widget|SetNationInformationListWidget _returnvalue)))
  (return (Variables|Widget|GetNationInformationListWidget)))

(fn PrepareNationManagement
  (Utilities|IsValid (Variables|Widget|GetNationManagementWidget)
    (:Is%20Valid
      _)
    (:Is%20Not%20Valid
      (bind _returnvalue (UserInterface|CreateWidget "/Game/UnrealDiplomacy/Skirmish/UI/WBP_NationManagement.WBP_NationManagement_C" (Game|GetPlayerController 0) 0))
      (bind _output_get (Variables|Widget|SetNationManagementWidget _returnvalue))
      (bind _returnvalue_2 (Game|ConstructObjectfromClass _output_get "/Script/UnrealDiplomacy.UDNationOverviewViewModel"))
      (Default|SetUDNationOverviewViewModel _output_get _returnvalue_2)))
  (return (Variables|Widget|GetNationManagementWidget)))

(fn DefineNationItemViewModels
  (bind _returnvalue (Class|UDActionAdministrator|GetPlayerList (Variables|Default|GetAction%20Model)))
  (for (_array_element _array_index) _returnvalue
    (if (Utilities|Array|IsValidIndex (Variables|Default|GetNationItemViewModels) _array_index)
      ;[1 1 1] Update existing
      (Class|UDNationItemViewModel|ChangeDisplayedNation (Utilities|Array|Get(acopy) (Variables|Default|GetNationItemViewModels) _array_index) (.Id (Utilities|Struct|BreakUDPlayerInfo _array_element)))
      (else
        ;[1 1 1] Create new view model as the current list is out of bounds...
        (bind _returnvalue_2 (Game|ConstructObjectfromClass self "/Script/UnrealDiplomacy.UDNationItemViewModel"))
        (bind _output_get (LocalVariables|SetCurrentViewModel _returnvalue_2))
        (Class|UDViewModelBase|SetAuthority _output_get (Variables|Default|GetAction%20Model))
        (Class|UDNationItemViewModel|ChangeDisplayedNation (LocalVariables|GetCurrentViewModel) (.Id (Utilities|Struct|BreakUDPlayerInfo _array_element)))
        (Utilities|Array|Add (Variables|Default|GetNationItemViewModels) (LocalVariables|GetCurrentViewModel)))))
  (return))

(fn OnUpdateNationItemViewModels
  (Default|UpdateNationItemViewModels (Variables|Widget|GetNationInformationListWidget) (Variables|Default|GetNationItemViewModels)))

(fn PrepareGlobalViewModels
  (Utilities|FlowControl|Sequence
    (:then_0
      (bind _returnvalue (Game|ConstructObjectfromClass self "/Script/UnrealDiplomacy.UDGoldInformationViewModel"))
      (Variables|Default|SetGoldInformationViewModel _returnvalue))
    (:then_1
      ;[1 1 1] dynamically adds missing members in update
      (Variables|Default|SetNationItemViewModels (Utilities|Array|MakeArray)))
    (:then_2
      (return))))

(fn HideLobby
  (Widget|RemovefromParent (Variables|Widget|GetLobbyWidget)))

(fn UpdateLobbySettings
  (params (Owner :type Integer) (Data :type FUD%20Lobby%20Settings%20Structure) (IsOwner :type Boolean))
  (Default|SetLobbySettings (Variables|Widget|GetLobbyWidget) Owner Data IsOwner)
  (return))

(fn UpdateLobbyPlayerSettings
  (params (NationSettings :type FUD%20Nation%20Settings%20Structure))
  (Default|SetLobbyPlayerSettings (Variables|Widget|GetLobbyWidget) NationSettings)
  (return))

(fn UpdateLobbyMembers
  (params (Members :type Array%20of%20FUD%20Player%20Data%20Structures))
  (Default|SetMembers (Variables|Widget|GetLobbyWidget) Members)
  (return))

(fn UpdateNationManagement
  (params (NationUniqueId :type Integer))
  (bind _nationmanagementwidget (Variables|Widget|GetNationManagementWidget))
  (Class|UDNationOverviewViewModel|SetSelectedNation (Variables|/Game/UnrealDiplomacy/Skirmish/UI/WBP_NationManagement.WBP_NationManagement_C|GetUDNationOverviewViewModel _nationmanagementwidget) NationUniqueId)
  (MatchUI|DisplayWidget _nationmanagementwidget)
  (return))

(fn UpdateTileManagement
  (params (Position :type Int%20Point%20Structure))
  (bind _tilemanegementwidget (Variables|Widget|GetTileManegementWidget))
  (Class|UDTileOverviewViewModel|SetSelectedPosition (Variables|/Game/UnrealDiplomacy/Skirmish/UI/WBP_TileManagement.WBP_TileManagement_C|GetUDTileOverviewViewModel _tilemanegementwidget) Position)
  (MatchUI|DisplayWidget _tilemanegementwidget)
  (return))

(fn SwitchMatchUI
  (params (MatchUI :type EUDMatchState%20Enum :default "NewEnumerator0"))
  (Utilities|FlowControl|Sequence
    (:then_0
      (MatchUI|ClearAllWidgets))
    (:then_1
      (switch Utilities|FlowControl|Switch|SwitchonEUDMatchState MatchUI
        (:NewEnumerator0
          (MatchUI|DisplayWidget (Variables|Widget|GetLobbyWidget)))
        (:NewEnumerator1
          (MatchUI|DisplayWidget (Variables|Widget|GetPlayerInformationBarWidget))
          (MatchUI|DisplayWidget (Variables|Widget|GetNationInformationListWidget))
          (MatchUI|DisplayWidget (Variables|Widget|GetTurnCounterWidget)))))
    (:then_2
      (return))))

(fn ClearAllWidgets
  ;[1 1 1] Comment
  (Utilities|FlowControl|Sequence
    (:then_0
      (MatchUI|HideWidget (Variables|Widget|GetLobbyWidget)))
    (:then_1
      (MatchUI|HideWidget (Variables|Widget|GetTurnCounterWidget)))
    (:then_4
      (return))))

(fn DisplayWidget
  (params (Target :type User%20Widget%20Object%20Reference))
  (if (UserInterface|Viewport|IsinViewport Target)
    _
    (else
      (UserInterface|Viewport|AddtoViewport Target 0)))
  (return))

(fn HideWidget
  (params (Target :type User%20Widget%20Object%20Reference))
  (if (UserInterface|Viewport|IsinViewport Target)
    (Widget|RemovefromParent Target))
  (return))