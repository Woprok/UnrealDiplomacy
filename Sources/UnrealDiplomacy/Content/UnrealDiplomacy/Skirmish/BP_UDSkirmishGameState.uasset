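; Replicated game state for an Unreal Diplomacy skirmish match, holding lobby settings, players, turn and hex tile data.
; Server events act as shortcuts from player controllers to the game mode, though surrender, leave and action validation are unfinished stubs.
; RepNotifies push updates to the local player controller, retrying each tick until it is valid.
; Toggled dirty-tag booleans trigger notifies for player and tile changes, refreshing UI and hex tile visuals.
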(event EventBeginPlay
  (CallFunction|LogInfo "GameStateBeginPlay" false))

(event Custom|OnServerStartGame
  ;[1 1 1] Represents shortcuts used for client calls, so Player Controller does not care about internal structure of GameState and GameMode
  (bind _asbp_udgame_mode (CallFunction|GetUDGameMode))
  (Default|StartGame _asbp_udgame_mode))

(event Custom|OnServerSurrenderGame
  ;[1 1 1] Represents shortcuts used for client calls, so Player Controller does not care about internal structure of GameState and GameMode
  (CallFunction|GetUDGameMode))

(event Custom|OnServerLeaveGame
  ;[1 1 1] Represents shortcuts used for client calls, so Player Controller does not care about internal structure of GameState and GameMode
  (CallFunction|GetUDGameMode))

(event Custom|OnServerUpdateLobbySettings
  (params (NewSettings :type FUD%20Lobby%20Settings%20Structure))
  ;[1 1 1] Update from user input
  (bind _asbp_udgame_mode (CallFunction|GetUDGameMode))
  (Default|UpdateLobbySettings _asbp_udgame_mode NewSettings))

(event Custom|OnServerUpdatePlayerSettings
  (params (Owner :type Integer) (NewNationSettings :type FUD%20Nation%20Settings%20Structure))
  ;[1 1 1] Update from user input
  (bind _asbp_udgame_mode (CallFunction|GetUDGameMode))
  (Default|UpdatePlayerSettings _asbp_udgame_mode Owner NewNationSettings))

(event Custom|OnServerEndTurn
  (params (CallerId :type Integer))
  ;[1 1 1] Update from user input
  (bind _asbp_udgame_mode (CallFunction|GetUDGameMode))
  (Default|PlayerEndTurn _asbp_udgame_mode CallerId))

(event Custom|OnServerExecuteAction
  (params (ExecutedActionData :type FUD%20Action%20Data%20Structure))
  ;[1 1 1] Update from user input
  (Utilities|IsValidAction ExecutedActionData
    (:Valid
      (bind _asbp_udgame_mode (CallFunction|GetUDGameMode))
      (Default|ExecuteAction _asbp_udgame_mode ExecutedActionData))))

(event Custom|ClientUpdateLobbyPlayerSettings
  ;[1 1 1] Server calls for updates to clients, based on certain criteria like replication notification.
  (bind _asbp_udplayer_controller (Utilities|ExecuteonValidClient)
    (:OnValidClient
      (Default|OnClientUpdateLobbyPlayerSettings _asbp_udplayer_controller (Helpers|GetPlayer (Variables|/Game/UnrealDiplomacy/Skirmish/BP_UDSkirmishPlayerController.BP_UDSkirmishPlayerController_C|GetAssignedUniqueId _asbp_udplayer_controller))))))

(event Custom|ClientUpdateLobbyMembers
  ;[1 1 1] Server calls for updates to clients, based on certain criteria like replication notification.
  (bind _asbp_udplayer_controller (Utilities|ExecuteonValidClient)
    (:OnValidClient
      (Default|OnClientUpdateLobbyMembers _asbp_udplayer_controller (Variables|GameControl|GetPlayers)))))

(event Custom|ClientUpdatePlayerResources
  ;[1 1 1] Server calls for updates to clients, based on certain criteria like replication notification.
  (bind _asbp_udplayer_controller (Utilities|ExecuteonValidClient)
    (:OnValidClient
      (Default|OnClientUpdatePlayerResources _asbp_udplayer_controller (Helpers|GetPlayer (Variables|/Game/UnrealDiplomacy/Skirmish/BP_UDSkirmishPlayerController.BP_UDSkirmishPlayerController_C|GetAssignedUniqueId _asbp_udplayer_controller))))))

(event Custom|ClientUpdateLobbySettings
  ;[1 1 1] Server calls for updates to clients, based on certain criteria like replication notification.
  (bind _asbp_udplayer_controller (Utilities|ExecuteonValidClient)
    (:OnValidClient
      (Default|OnClientUpdateLobbySettings _asbp_udplayer_controller (Variables|GameControl|GetCurrentGameOwner) (Variables|GameControl|GetCurrentGameLobby)))))

(event Custom|ClientUpdateNations
  ;[1 1 1] Server calls for updates to clients, based on certain criteria like replication notification.
  (bind _asbp_udplayer_controller (Utilities|ExecuteonValidClient)
    (:OnValidClient
      (Default|OnClientUpdateNations _asbp_udplayer_controller (Variables|GameControl|GetPlayers)))))

(event Custom|ClientUpdateMatchStateUI
  ;[1 1 1] Server calls for updates to clients, based on certain criteria like replication notification.
  (bind _asbp_udplayer_controller (Utilities|ExecuteonValidClient)
    (:OnValidClient
      (Default|OnClientUpdateMatchStateUI _asbp_udplayer_controller (Variables|GameControl|GetCurrentGameState)))))

(event Custom|ClientUpdateTurnData
  (bind _currentturn (Variables|GameControl|GetCurrentTurn))
  ;[1 1 1] Server calls for updates to clients, based on certain criteria like replication notification.
  (bind _asbp_udplayer_controller (Utilities|ExecuteonValidClient)
    (:OnValidClient
      (Default|OnClientUpdateTurnData _asbp_udplayer_controller _currentturn (== (Variables|/Game/UnrealDiplomacy/Skirmish/BP_UDSkirmishPlayerController.BP_UDSkirmishPlayerController_C|GetAssignedUniqueId _asbp_udplayer_controller) (.PlayerUniqueId (Utilities|Struct|BreakFUDTurnData _currentturn)))))))

(event Custom|ClientNotifyTileActionExecuted
  (params (TileIndices :type Int%20Point%20Structure) (TileData :type UD%20Tile%20Structure))
  (bind _asbp_udplayer_controller (Utilities|ExecuteonValidClient)
    (:OnValidClient
      (CallFunction|LogInfo (Utilities|String|ToString(Integer) (.Owner (Utilities|Struct|BreakUDTile TileData))) true)
      (Default|OnClientUpdateTile _asbp_udplayer_controller TileIndices TileData))))

(event Custom|ClientSimulationStep
  (params (SimulationStep :type FUD%20Action%20Data%20Structure))
  ;[1 1 1] Server calls for updates to clients, based on certain criteria like replication notification.
  (bind _asbp_udplayer_controller (Utilities|ExecuteonValidClient)
    (:OnValidClient
      (Default|OnClientSimulationStep _asbp_udplayer_controller SimulationStep))))

(fn ConstructionScript
  (CallFunction|LogInfo "GameStateConstruct" false)
  ;[1 1 1] Initialize Game State (this is used to setup real values and force sync to always happen)
  (Variables|GameControl|SetCurrentGameOwner -1)
  (Variables|GameControl|SetCurrentGameState "NewEnumerator0")
  (Variables|GameControl|SetCurrentGameLobby (Utilities|Struct|MakeFUDLobbySettings))
  (Variables|GameControl|SetCurrentTurn (Utilities|Struct|MakeFUDTurnData)))

(fn CreateNewPlayer
  (params (UniqueId :type Integer))
  (Utilities|Array|Add (Variables|GameControl|GetPlayers) (Utilities|Struct|MakeFUDPlayerData UniqueId (Utilities|String|Append "Player " (Utilities|String|ToString(Integer) UniqueId)) "NewEnumerator1" "NewEnumerator1" (CallFunction|RetrieveDefaultResources) (CallFunction|RetrieveDefaultNation UniqueId)))
  (Utilities|UpdatePlayersTag
    (:Execute
      (return))))

(fn UpdatePlayerSettings
  (params (Owner :type Integer) (NewNationSettngs :type FUD%20Nation%20Settings%20Structure))
  (bind _players (Variables|GameControl|GetPlayers))
  (bind (_array_element _array_index) (Utilities|Array|ForEachLoopwithBreak _players :!label _label)
    (:LoopBody
      (if (== Owner (.UniqueId (Utilities|Struct|BreakFUDPlayerData _array_element)))
        (goto _label Break)))
    (:Completed
      (bind _structout (Utilities|Struct|SetmembersinFUDPlayerData _array_element NewNationSettngs))
      (Utilities|Array|SetArrayElem _players _array_index _structout)
      (CallFunction|LogInfo (Utilities|String|Append "P: " (Utilities|String|ToString(Integer) (.UniqueId (Utilities|Struct|BreakFUDPlayerData (Utilities|Array|Get(acopy) (Variables|GameControl|GetPlayers) _array_index)))) "," (.Name (Utilities|Struct|BreakFUDNationSettings (.Nation (Utilities|Struct|BreakFUDPlayerData (Utilities|Array|Get(acopy) (Variables|GameControl|GetPlayers) _array_index))))) ",  " (Utilities|Struct|BreakUDTileRegion (.Region (Utilities|Struct|BreakFUDNationSettings (.Nation (Utilities|Struct|BreakFUDPlayerData (Utilities|Array|Get(acopy) (Variables|GameControl|GetPlayers) _array_index)))))) ",  " (Utilities|Struct|BreakUDTileBiome (.Biome (Utilities|Struct|BreakFUDNationSettings (.Nation (Utilities|Struct|BreakFUDPlayerData (Utilities|Array|Get(acopy) (Variables|GameControl|GetPlayers) _array_index)))))) ",  " (Utilities|Struct|BreakUDTileFeature (.Feature (Utilities|Struct|BreakFUDNationSettings (.Nation (Utilities|Struct|BreakFUDPlayerData (Utilities|Array|Get(acopy) (Variables|GameControl|GetPlayers) _array_index))))))) true)
      (Utilities|UpdatePlayersTag
        (:Execute
          (return))))))

(fn UpdateTilesData
  (Utilities|UpdateTilesTag
    (:Execute
      (return))))

(fn CreateNewSpectator
  (params (UniqueId :type Integer))
  (Utilities|Array|Add (Variables|GameControl|GetPlayers) (Utilities|Struct|MakeFUDPlayerData UniqueId "Spectator" "NewEnumerator6"))
  (Utilities|UpdatePlayersTag
    (:Execute
      (return))))

(fn OnRepCurrentGameOwner
  (CallFunction|ClientUpdateLobbySettings)
  (return))

(fn OnRepCurrentGameState
  (CallFunction|ClientUpdateMatchStateUI)
  (return))

(fn OnRepCurrentGameLobby
  (CallFunction|ClientUpdateLobbySettings)
  (return))

(fn OnRepPlayers
  ;[1 1 1] This update should be not needed as Dirty Tag should always be updated
  (CallFunction|PlayersonRepCollection)
  (return))

(fn OnRepPlayersDirtyTag
  (CallFunction|PlayersonRepCollection)
  (return))

(fn GetPlayer
  (params (AssignedId :type Integer))
  ;[1 1 1] Searched player should always exists
  (bind _array_element (Utilities|Array|ForEachLoopwithBreak (Variables|GameControl|GetPlayers) :!label _label)
    (:LoopBody
      (if (== (.UniqueId (Utilities|Struct|BreakFUDPlayerData _array_element)) AssignedId)
        (goto _label Break)))
    (:Completed
      (return _array_element))))

(fn OnRepCurrentTurn
  (CallFunction|ClientUpdateTurnData)
  (return))

(fn PlayersonRepCollection
  (Utilities|FlowControl|Sequence
    (:then_0
      (CallFunction|ClientUpdateLobbyMembers))
    (:then_1
      (CallFunction|ClientUpdateLobbyPlayerSettings))
    (:then_2
      (CallFunction|ClientUpdatePlayerResources))
    (:then_3
      (CallFunction|ClientUpdateNations))
    (:then_4
      (return))))

(fn GetTileInfo
  (params (TileIndices :type Int%20Point%20Structure) (RequesterId :type Integer))
  (bind (_x _y) (Utilities|Struct|BreakIntPoint TileIndices))
  (if (Utilities|Array|IsValidIndex (Variables|GameControl|GetTileData) _x)
    (if (Utilities|Array|IsValidIndex (Utilities|Struct|BreakUDTileRow (Utilities|Array|Get(acopy) (Variables|GameControl|GetTileData) _x)) _y)
      (return (Utilities|Array|Get(acopy) (Utilities|Struct|BreakUDTileRow (Utilities|Array|Get(acopy) (Variables|GameControl|GetTileData) _x)) _y) (Utilities|Array|MakeArray (Utilities|Struct|MakeFUDActionData "Claim" "/Game/UnrealDiplomacy/Development/Data/Icons/ActionIcon.ActionIcon" RequesterId "NewEnumerator0" (Utilities|Array|MakeArray TileIndices))))
      (else
        _)))
  ;[1 1 1] Fake result for unsynchronzid access
  (return (Utilities|Struct|MakeUDTile 0 "(Name=\"\")" "(Name=\"\")" (Utilities|Array|MakeArray "") (Utilities|Array|MakeArray "")) (Utilities|Array|MakeArray "")))

(fn OnRepTilesDirtyTag
  (bind _outactors (Actor|GetAllActorsOfClass "/Game/UnrealDiplomacy/Development/HexTiles/BP_AUDHexTile.BP_AUDHexTile_C"))
  (for _array_element _outactors
    (Default|RefreshVisuals _array_element)
    (CallFunction|ClientNotifyTileActionExecuted (Variables|/Script/UnrealDiplomacy.UDHexTile|GetDataIndices _array_element))))

(fn OnRepActionDirtyTag)

(fn UpdateAction
  (Utilities|UpdateActionTag
    (:Execute
      (return))))