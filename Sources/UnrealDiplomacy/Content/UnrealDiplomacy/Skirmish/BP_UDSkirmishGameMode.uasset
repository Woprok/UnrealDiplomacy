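; Server game mode for an UnrealDiplomacy skirmish that runs the lobby, turn order and player actions.
; Joining controllers get sequential IDs and become players in the lobby, the first as game owner, or spectators afterwards.
; StartGame builds turn order from active players; turn endings and tile claims update the shared game state.
; Construction spawns a server simulation manager; logout only logs, while surrender and leave are empty.
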(event EventBeginPlay
  ;[1 1 1] BeginPlay is unreliable as it happens after OnPostLogin.
  (CallFunction|LogInfo "GameModeBeginPlay" false))

(event EventPostLogin
  (params (NewPlayer :type Player%20Controller%20Object%20Reference))
  ;[1 1 1] OnPostLogin happens everytime new client joins the session.
  (CallFunction|LogInfo "GameModeOnPostLogin" false)
  ;[1 1 1] Each player that joins will be assigned Id from 0 to INT32.MAX
  (bind _asbp_udskirmish_player_controller (Utilities|Casting|CastToBP_UDSkirmishPlayerController NewPlayer))
  (bind _new_player_id (Initialization|AssignUniqueId _asbp_udskirmish_player_controller))
  ;[1 1 1] Create Player Data that will be saved in Game State for everyone to read access.
  (bind _asbp_udgame_state (CallFunction|GetUDGameState))
  (Utilities|IsinLobby
    (:True
      (Default|CreateNewPlayer _asbp_udgame_state _new_player_id)
      (Initialization|AssignGameOwner _new_player_id))
    (:False
      (Default|CreateNewSpectator _asbp_udgame_state _new_player_id))))

(event EventOnLogout
  (params (ExitingController :type Controller%20Object%20Reference))
  ;[1 1 1] TODO: Allow players to claim nation of player that left (useful for reconnect) + HANDLE DISCONNECT
  (bind _asbp_udskirmish_player_controller (Utilities|Casting|CastToBP_UDSkirmishPlayerController ExitingController))
  (CallFunction|LogInfo (Utilities|String|ToString(Integer) (Variables|/Game/UnrealDiplomacy/Skirmish/BP_UDSkirmishPlayerController.BP_UDSkirmishPlayerController_C|GetAssignedUniqueId _asbp_udskirmish_player_controller)) true))

(event Custom|SurrenderGame
  ;[1 1 1] Comment
)

(event Custom|StartGame
  ;[1 1 1] Comment
  (Utilities|IsinLobby
    (:True
      (bind _asbp_udgame_state (CallFunction|GetUDGameState))
      (Variables|/Game/UnrealDiplomacy/Skirmish/BP_UDSkirmishGameState.BP_UDSkirmishGameState_C|SetCurrentGameState _asbp_udgame_state "NewEnumerator1")
      (CallFunction|CreateStart)
      (CallFunction|CreateTurnOrder))
    (:False
      (CallFunction|LogError "Can't start game twice." true))))

(event Custom|LeaveGame
  ;[1 1 1] Comment
)

(event Custom|UpdateLobbySettings
  (params (CurrentGameLobby :type FUD%20Lobby%20Settings%20Structure))
  ;[1 1 1] Comment
  (bind _asbp_udgame_state (CallFunction|GetUDGameState))
  (Variables|/Game/UnrealDiplomacy/Skirmish/BP_UDSkirmishGameState.BP_UDSkirmishGameState_C|SetCurrentGameLobby _asbp_udgame_state CurrentGameLobby))

(event Custom|UpdatePlayerSettings
  (params (Owner :type Integer) (NewNationSettngs :type FUD%20Nation%20Settings%20Structure))
  ;[1 1 1] Comment
  (bind _asbp_udgame_state (CallFunction|GetUDGameState))
  (Default|UpdatePlayerSettings _asbp_udgame_state Owner NewNationSettngs))

(event Custom|PlayerEndTurn
  (params (PlayerId :type Integer))
  ;[1 1 1] Comment
  (CallFunction|ResolveTurn PlayerId))

(event Custom|ExecuteAction
  (params (ActionData :type FUD%20Action%20Data%20Structure))
  ;[1 1 1] Comment
  (CallFunction|ResolveAction ActionData))

(fn ConstructionScript
  ;[1 1 1] Initialize Game Mode State (this is not necessary to do (var defaults), but its done for clarity)
  (CallFunction|LogInfo "GameModeConstruct" false)
  (bind _simulationmanager (Initialization|CreateSimulation 0 false true))
  (bind _output_get (Variables|Default|SetServerSimulation _simulationmanager))
  (Default|CreateWorldPlayer _output_get))

(fn CreateSimulation
  (params (Owner :type Actor%20Object%20Reference) (IsWorldVisible :type Boolean) (IsComplete :type Boolean))
  (bind _returnvalue (Game|SpawnActorfromClass "/Game/UnrealDiplomacy/Core/Managers/BP_AUDGameSimulationManager.BP_AUDGameSimulationManager_C" (Math|Conversions|ToTransform(Vector) "0, 0, 0") "Undefined" Owner 0))
  (Variables|/Game/UnrealDiplomacy/Core/Managers/BP_AUDGameSimulationManager.BP_AUDGameSimulationManager_C|SetIsWorldVisible _returnvalue IsWorldVisible)
  (Variables|/Game/UnrealDiplomacy/Core/Managers/BP_AUDGameSimulationManager.BP_AUDGameSimulationManager_C|SetIsComplete _returnvalue IsComplete)
  (return _returnvalue))

(fn AssignGameOwner
  (params (PlayerUniqueId :type Integer))
  (bind _asbp_udgame_state (CallFunction|GetUDGameState))
  (if (== (Variables|/Game/UnrealDiplomacy/Skirmish/BP_UDSkirmishGameState.BP_UDSkirmishGameState_C|GetCurrentGameOwner _asbp_udgame_state) -1)
    (Variables|/Game/UnrealDiplomacy/Skirmish/BP_UDSkirmishGameState.BP_UDSkirmishGameState_C|SetCurrentGameOwner _asbp_udgame_state PlayerUniqueId))
  (return))

(fn AssignUniqueId
  (params (New%20Player :type BP%20UD%20Skirmish%20Player%20Controller%20Object%20Reference))
  ;[1 1 1] Assign unique ID to player for future identification. Starts at -1, so first is always 0.
  (bind _result (Math|Integer|IncrementInt (Variables|GameControl|GetNextPlayerUniqueId))
    (:%20%20
      (bind _output_get (Variables|/Game/UnrealDiplomacy/Skirmish/BP_UDSkirmishPlayerController.BP_UDSkirmishPlayerController_C|SetAssignedUniqueId New%20Player _result))
      (return _output_get))))

(fn CreateStart
  (Utilities|FlowControl|Sequence
    (:then_1
      (bind _asbp_udgame_state (CallFunction|GetUDGameState))
      (Default|UpdateTilesData _asbp_udgame_state))
    (:then_2
      (return))))

(fn ResolveTurn
  (params (PlayerId :type Integer))
  (bind _player (CallFunction|RetrievePlayeratCurrentTurnOrder))
  (bind (_uniqueid _name) (Utilities|Struct|BreakFUDPlayerData _player))
  (bind _asbp_udgame_state (CallFunction|GetUDGameState))
  (if (== PlayerId (.PlayerUniqueId (Utilities|Struct|BreakFUDTurnData (Variables|/Game/UnrealDiplomacy/Skirmish/BP_UDSkirmishGameState.BP_UDSkirmishGameState_C|GetCurrentTurn _asbp_udgame_state))))
    (Utilities|FlowControl|Sequence
      (:then_0
        ;[1 1 1] Increment current index
        (bind _result (Math|Integer|IncrementInt (Variables|GameControl|GetTurnOrderIndex))
          (:%20%20
            (if (>= _result (Utilities|Array|Length (Variables|GameControl|GetTurnOrderToPlayersIndices)))
              (Variables|GameControl|SetTurnOrderIndex 0)))))
      (:then_1
        ;[1 1 1] Get reference index to Players and get that player. Finally update turn to next player and let it be propagated by notify
        (bind _result_2 (Math|Integer|IncrementInt (.Turn (Utilities|Struct|BreakFUDTurnData (Variables|/Game/UnrealDiplomacy/Skirmish/BP_UDSkirmishGameState.BP_UDSkirmishGameState_C|GetCurrentTurn _asbp_udgame_state))))
          (:%20%20
            (Variables|/Game/UnrealDiplomacy/Skirmish/BP_UDSkirmishGameState.BP_UDSkirmishGameState_C|SetCurrentTurn _asbp_udgame_state (Utilities|Struct|MakeFUDTurnData _result_2 _uniqueid _name))
            (return)))))
    (else
      (CallFunction|LogError "Out of turn order end turn request." true)
      (return))))

(fn CreateTurnOrder
  (bind _player (CallFunction|RetrievePlayeratCurrentTurnOrder))
  (bind (_uniqueid _name) (Utilities|Struct|BreakFUDPlayerData _player))
  ;[1 1 1] Create turn order from living players as an array of pure index to their array for fast access, repeated calls will rebuilt it but maintain current turnorder player
  (if (!= (Variables|GameControl|GetTurnOrderIndex) -1)
    _
    (else
      (LocalVariables|SetBackupPlayerIndex (Utilities|Array|Get(acopy) (Variables|GameControl|GetTurnOrderToPlayersIndices) (Variables|GameControl|GetTurnOrderIndex)))))
  (Utilities|Array|Clear (Variables|GameControl|GetTurnOrderToPlayersIndices))
  (bind _asbp_udgame_state (CallFunction|GetUDGameState))
  (for (_array_element _array_index) (Variables|/Game/UnrealDiplomacy/Skirmish/BP_UDSkirmishGameState.BP_UDSkirmishGameState_C|GetPlayers _asbp_udgame_state)
    (if (Utilities|Enum|Equal(Enum) (.GameStatus (Utilities|Struct|BreakFUDPlayerData _array_element)) "NewEnumerator1")
      (Utilities|Array|Add (Variables|GameControl|GetTurnOrderToPlayersIndices) _array_index)))
  (if (== (Variables|GameControl|GetTurnOrderIndex) -1)
    (Variables|GameControl|SetTurnOrderIndex 0)
    (Variables|/Game/UnrealDiplomacy/Skirmish/BP_UDSkirmishGameState.BP_UDSkirmishGameState_C|SetCurrentTurn _asbp_udgame_state (Utilities|Struct|MakeFUDTurnData 0 _uniqueid _name))
    (return)
    (else
      (bind (_array_element_2 _array_index_2) (Utilities|Array|ForEachLoopwithBreak (Variables|GameControl|GetTurnOrderToPlayersIndices) :!label _label)
        (:LoopBody
          (if (== _array_element_2 (LocalVariables|GetBackupPlayerIndex))
            (Variables|GameControl|SetTurnOrderIndex _array_index_2)
            (goto _label Break)))
        (:Completed
          (return))))))

(fn RetrievePlayeratCurrentTurnOrder
  (bind _asbp_udgame_state (CallFunction|GetUDGameState))
  (return (Utilities|Array|Get(acopy) (Variables|/Game/UnrealDiplomacy/Skirmish/BP_UDSkirmishGameState.BP_UDSkirmishGameState_C|GetPlayers _asbp_udgame_state) (Utilities|Array|Get(acopy) (Variables|GameControl|GetTurnOrderToPlayersIndices) (Variables|GameControl|GetTurnOrderIndex)))))

(fn ResolveAction
  (params (ActionData :type FUD%20Action%20Data%20Structure))
  (bind (_name _invokerid _targettype _tileindices) (Utilities|Struct|BreakFUDActionData ActionData))
  (switch string _name
    (:Claim
      (bind _asbp_udgame_state (CallFunction|GetUDGameState))
      (for _array_element _tileindices
        (Utilities|Struct|SetmembersinUDTile (Utilities|Array|Get(acopy) (Utilities|Struct|BreakUDTileRow (Utilities|Array|Get(acopy) (Variables|/Game/UnrealDiplomacy/Skirmish/BP_UDSkirmishGameState.BP_UDSkirmishGameState_C|GetTileData _asbp_udgame_state) (.X (Utilities|Struct|BreakIntPoint _array_element)))) (.Y (Utilities|Struct|BreakIntPoint _array_element))) _invokerid)
        (bind _asbp_udgame_state_2 (CallFunction|GetUDGameState))
        (Default|UpdateAction _asbp_udgame_state_2)
        (CallFunction|LogInfo (Utilities|String|ToString(Integer) (.Owner (Utilities|Struct|BreakUDTile (Utilities|Array|Get(acopy) (Utilities|Struct|BreakUDTileRow (Utilities|Array|Get(acopy) (Variables|/Game/UnrealDiplomacy/Skirmish/BP_UDSkirmishGameState.BP_UDSkirmishGameState_C|GetTileData _asbp_udgame_state) (.X (Utilities|Struct|BreakIntPoint _array_element)))) (.Y (Utilities|Struct|BreakIntPoint _array_element)))))) true)
        (Default|ClientNotifyTileActionExecuted _asbp_udgame_state_2 _array_element (Utilities|Array|Get(acopy) (Utilities|Struct|BreakUDTileRow (Utilities|Array|Get(acopy) (Variables|/Game/UnrealDiplomacy/Skirmish/BP_UDSkirmishGameState.BP_UDSkirmishGameState_C|GetTileData _asbp_udgame_state) (.X (Utilities|Struct|BreakIntPoint _array_element)))) (.Y (Utilities|Struct|BreakIntPoint _array_element))))))))