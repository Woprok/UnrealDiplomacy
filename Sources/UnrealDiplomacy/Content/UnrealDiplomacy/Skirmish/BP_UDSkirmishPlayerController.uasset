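; Skirmish player controller for UnrealDiplomacy that links lobby and match updates to the client's HUD and square grid.
; Client events forward lobby and match data to the HUD, flagging lobby ownership by player ID.
; Synchronization binds HUD models to the personal administrator; world-state changes refresh models and grid, while selection changes pass to the HUD.
; UI actions go out through ServercastSendActionToServer; the Server-prefixed events here are empty stubs.
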(event Custom|ServerUpdateLobbySettings
  (params (NewSettings :type FUD%20Lobby%20Settings%20Structure))
  ;[1 1 1] Represents calls that client needs to execute on server like actions. Actions can be for example End Turn, Build, Diplomacy etc.
)

(event Custom|ServerLeaveGame
  ;[1 1 1] Provides calls that GameInstance needs to invoke on the Server such as Start, Surrender and Leave Game.
)

(event Custom|ServerUpdateLobbyPlayerSettings
  (params (NewNationSettings :type FUD%20Nation%20Settings%20Structure))
  ;[1 1 1] Represents calls that client needs to execute on server like actions. Actions can be for example End Turn, Build, Diplomacy etc.
)

(event Custom|ServerSurrenderGame
  ;[1 1 1] Provides calls that GameInstance needs to invoke on the Server such as Start, Surrender and Leave Game.
)

(event Custom|ServerExecuteAction
  (params (ActionData :type FUD%20Action%20Data%20Structure))
  ;[1 1 1] Represents calls that client needs to execute on server like actions. Actions can be for example End Turn, Build, Diplomacy etc.
)

(event Custom|OnClientUpdateLobbyPlayerSettings
  (params (Player :type FUD%20Player%20Data%20Structure))
  ;[1 1 1] Provides events that are used to notify this player controller that some data have changed and this instance should update this client.
  (bind _asbp_udhud (CallFunction|GetUDHUD))
  (Default|OnUpdateLobbyPlayerSettings _asbp_udhud (.Nation (Utilities|Struct|BreakFUDPlayerData Player))))

(event Custom|OnClientUpdateLobbySettings
  (params (Owner :type Integer) (LobbyData :type FUD%20Lobby%20Settings%20Structure))
  ;[1 1 1] Provides events that are used to notify this player controller that some data have changed and this instance should update this client.
  (bind _asbp_udhud (CallFunction|GetUDHUD))
  (Default|OnUpdateLobbySettings _asbp_udhud Owner LobbyData (CallFunction|IsOwner Owner)))

(event Custom|OnClientUpdateLobbyMembers
  (params (Members :type Array%20of%20FUD%20Player%20Data%20Structures))
  ;[1 1 1] Provides events that are used to notify this player controller that some data have changed and this instance should update this client.
  (bind _asbp_udhud (CallFunction|GetUDHUD))
  (Default|OnUpdateLobbyMembers _asbp_udhud Members))

(event Custom|OnClientUpdateMatchStateUI
  (params (MatchUI :type EUDMatchState%20Enum :default "NewEnumerator0"))
  ;[1 1 1] Provides events that are used to notify this player controller that some data have changed and this instance should update this client.
  (bind _asbp_udhud (CallFunction|GetUDHUD))
  (Default|OnUpdateMatchStateUI _asbp_udhud MatchUI))

(event Custom|ActionExecutedByUI
  (params (ActionData :type UD%20Action%20Data%20Structure))
  ;[1 1 1] C++ calls resolutions
  (Class|UDSkirmishPlayerController|ServercastSendActiontoServer ActionData))

(event Custom|OnTileSelectionChanged
  (params (Position :type Int%20Point%20Structure))
  (CallFunction|LogInfo "Tile Selection changed." true)
  (bind _asbp_udhud (CallFunction|GetUDHUD))
  (Default|TileSelectionChanged _asbp_udhud Position))

(event Custom|OnNationSelectionChanged
  (params (PlayerUniqueId :type Integer))
  (CallFunction|LogInfo "Nation Selection Changed." true)
  (bind _asbp_udhud (CallFunction|GetUDHUD))
  (Default|NationSelectionChanged _asbp_udhud PlayerUniqueId))

(event EventOnSynchronizationFinished
  ;[1 1 1] C++ calls resolutions
  (CallFunction|LogInfo "Synchronization for widgets started." true)
  (bind _asbp_udhud (CallFunction|GetUDHUD))
  (bind _returnvalue (Class|UDSkirmishPlayerController|GetPersonalAdministrator))
  (Default|BindModels _asbp_udhud _returnvalue)
  (Default|UpdateModels _asbp_udhud)
  (Class|UDSquareGrid|OnUpdate (Variables|Default|GetSquareGrid)))

(event EventOnWorldStateUpdated
  ;[1 1 1] C++ calls resolutions
  (CallFunction|LogInfo "World state updated." true)
  (bind _asbp_udhud (CallFunction|GetUDHUD))
  (Default|UpdateModels _asbp_udhud)
  (Class|UDSquareGrid|OnUpdate (Variables|Default|GetSquareGrid)))

(fn ConstructionScript
  (CallFunction|LogInfo "BP_UDSkirmishPlayerController: Construction Script." false))

(fn IsOwner
  (params (OwnerId :type Integer))
  (return (== OwnerId (Variables|Default|GetAssignedUniqueId))))