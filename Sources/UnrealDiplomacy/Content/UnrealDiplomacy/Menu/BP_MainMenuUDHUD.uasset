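; Client-only main menu HUD for Unreal Diplomacy that owns and switches between the main, join game, options and credits screens.
; The construction script pre-creates each widget through lazy Prepare functions, and Switch functions clear the viewport before adding the requested one.
; Menu button callbacks route through InvokeOn events, which switch screens or call the UD GameInstance to host, search, join, start the tutorial or quit.
; GameInstance session search results are forwarded to the join game widget.
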(event Custom|OnValidSessionList
  (params (Sessions :type Array%20of%20Blueprint%20Session%20Result%20Structures))
  ;[1 1 1] Initialization, this is client only HUD, so there is no need for preemptive initialization in constructor
  ;;[1 1 1] Initialize Join Game
  (Default|OnSearchwithValidList (Variables|Widgets|GetJoinGameMenuWidget) Sessions))

(event Custom|OnEmptySessionList
  ;[1 1 1] Initialization, this is client only HUD, so there is no need for preemptive initialization in constructor
  ;;[1 1 1] Initialize Join Game
  (Default|OnSearchwithInvalidList (Variables|Widgets|GetJoinGameMenuWidget)))

(event EventBeginPlay
  ;[1 1 1] Initialization, this is client only HUD, so there is no need for preemptive initialization in constructor
  (Utilities|FlowControl|Sequence
    (:then_0
      ;;[1 1 1] Initialize Join Game
      (bind _asbp_uudgame_instance (CallFunction|GetUDGameInstance))
      (EventDispatchers|BindEventtoOnValidSessionList _asbp_uudgame_instance (delegate Custom|OnValidSessionList))
      (EventDispatchers|BindEventtoOnEmptySessionList _asbp_uudgame_instance (delegate Custom|OnEmptySessionList)))
    (:then_1
      ;;[1 1 1] Progress to initial UI
      (Widgets|SwitchtoMainMenu)
      (Class|UDHUD|CreateWidgets)
      (Class|UDHUD|ShowWidgets)
      (Class|UDHUD|CreateViewModels)
      (Class|UDHUD|BindViewModel)
      (Class|UDHUD|UpdateViewModel))))

(event Custom|InvokeOnBackClicked
  ;[1 1 1] All callbacks from Menu UI elements are required to go through here
  (Widgets|SwitchtoMainMenu))

(event Custom|InvokeOnOptionsClicked
  ;[1 1 1] All callbacks from Menu UI elements are required to go through here
  (Widgets|SwitchtoOptionsMenuandLoad))

(event Custom|InvokeOnHostClicked
  ;[1 1 1] All callbacks from Menu UI elements are required to go through here
  (bind _asbp_uudgame_instance (CallFunction|GetUDGameInstance))
  (Default|CreateGame _asbp_uudgame_instance))

(event Custom|InvokeOnSaveSettingsClicked
  ;[1 1 1] All callbacks from Menu UI elements are required to go through here
  ;;[0 1 0] Actions for options
  (Widgets|SwitchtoMainMenu))

(event Custom|InvokeOnJoinClicked
  ;[1 1 1] All callbacks from Menu UI elements are required to go through here
  ;;[0 1 0] Actions for join game
  (Widgets|SwitchtoJoinGameMenu))

(event Custom|InvokeOnTutorialClicked
  ;[1 1 1] All callbacks from Menu UI elements are required to go through here
  (bind _asbp_uudgame_instance (CallFunction|GetUDGameInstance))
  (Default|CreateTutorialGame _asbp_uudgame_instance))

(event Custom|InvokeOnQuitClicked
  ;[1 1 1] All callbacks from Menu UI elements are required to go through here
  (bind _asbp_uudgame_instance (CallFunction|GetUDGameInstance))
  (Default|QuitfromMainMenu _asbp_uudgame_instance))

(event Custom|InvokeOnSearchForGamesClicked
  ;[1 1 1] All callbacks from Menu UI elements are required to go through here
  ;;[0 1 0] Actions for join game
  (bind _asbp_uudgame_instance (CallFunction|GetUDGameInstance))
  (Default|SearchforGames _asbp_uudgame_instance))

(event Custom|InvokeOnCreditsClicked
  ;[1 1 1] All callbacks from Menu UI elements are required to go through here
  (Widgets|SwitchtoCreditsMenu))

(event Custom|InvokeOnJoinGameClicked
  (params (SearchResult :type Blueprint%20Session%20Result%20Structure%20%28by%20ref%29))
  ;[1 1 1] All callbacks from Menu UI elements are required to go through here
  (bind _asbp_uudgame_instance (CallFunction|GetUDGameInstance))
  (Default|JoinGame _asbp_uudgame_instance SearchResult))

(fn ConstructionScript
  ;[1 1 1] Create all UI elements in advance
  (Utilities|FlowControl|Sequence
    (:then_0
      (Widgets|PrepareJoinGameMenu))
    (:then_1
      (Widgets|PrepareMainMenu))
    (:then_2
      (Widgets|PrepareCreditsMenu))
    (:then_3
      (Widgets|PrepareOptionsMenu))))

(fn PrepareJoinGameMenu
  (Utilities|IsValid (Variables|Widgets|GetJoinGameMenuWidget)
    (:Is%20Valid
      _)
    (:Is%20Not%20Valid
      (bind _returnvalue (UserInterface|CreateWidget "/Game/UnrealDiplomacy/Menu/UI/WBP_JoinGameMenu.WBP_JoinGameMenu_C" (Game|GetPlayerController 0)))
      (Variables|Widgets|SetJoinGameMenuWidget _returnvalue)))
  (return (Variables|Widgets|GetJoinGameMenuWidget)))

(fn PrepareCreditsMenu
  (Utilities|IsValid (Variables|Widgets|GetCreditsMenuWidget)
    (:Is%20Valid
      _)
    (:Is%20Not%20Valid
      (bind _returnvalue (UserInterface|CreateWidget "/Game/UnrealDiplomacy/Menu/UI/WBP_CreditsMenu.WBP_CreditsMenu_C" (Game|GetPlayerController 0)))
      (Variables|Widgets|SetCreditsMenuWidget _returnvalue)))
  (return (Variables|Widgets|GetCreditsMenuWidget)))

(fn PrepareMainMenu
  (Utilities|IsValid (Variables|Widgets|GetMainMenuWidget)
    (:Is%20Valid
      _)
    (:Is%20Not%20Valid
      (bind _returnvalue (UserInterface|CreateWidget "/Game/UnrealDiplomacy/Menu/UI/WBP_MainMenu.WBP_MainMenu_C" (Game|GetPlayerController 0)))
      (Variables|Widgets|SetMainMenuWidget _returnvalue)))
  (return (Variables|Widgets|GetMainMenuWidget)))

(fn PrepareOptionsMenu
  (Utilities|IsValid (Variables|Widgets|GetOptionsMenuWidget)
    (:Is%20Valid
      _)
    (:Is%20Not%20Valid
      (bind _returnvalue (UserInterface|CreateWidget "/Game/UnrealDiplomacy/Menu/UI/WBP_OptionsMenu.WBP_OptionsMenu_C" (Game|GetPlayerController 0)))
      (Variables|Widgets|SetOptionsMenuWidget _returnvalue)))
  (return (Variables|Widgets|GetOptionsMenuWidget)))

(fn SwitchtoJoinGameMenu
  (Viewport|RemoveAllWidgets)
  (bind _joingamewidget (Widgets|PrepareJoinGameMenu))
  (UserInterface|Viewport|AddtoViewport _joingamewidget 0)
  (return))

(fn SwitchtoOptionsMenuandLoad
  (Viewport|RemoveAllWidgets)
  (bind _optionswidget (Widgets|PrepareOptionsMenu))
  (Default|LoadSettings _optionswidget)
  (UserInterface|Viewport|AddtoViewport _optionswidget 0)
  (return))

(fn SwitchtoMainMenu
  (Viewport|RemoveAllWidgets)
  (bind _mainmenuwidget (Widgets|PrepareMainMenu))
  (UserInterface|Viewport|AddtoViewport _mainmenuwidget 0)
  (return))

(fn SwitchtoCreditsMenu
  (Viewport|RemoveAllWidgets)
  (bind _creditswidget (Widgets|PrepareCreditsMenu))
  (UserInterface|Viewport|AddtoViewport _creditswidget 0)
  (return))