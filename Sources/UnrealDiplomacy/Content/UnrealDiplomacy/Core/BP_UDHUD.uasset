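; HUD for UnrealDiplomacy that owns the lobby, current-player list and turn counter widgets.
; On BeginPlay it sets the application state on the game instance, lazily creates each widget, and shows the lobby (enabled only with authority) and player list.
; UI callbacks route through it: quit and start go to the game instance, end turn to the player controller, and turn events show or update the counter.
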(event EventBeginPlay
  ;[1 1 1] Any time level is loaded
  (bind _asbp_uudgame_instance (Utilities|GetGameInstance))
  (Default|SetApplicationState _asbp_uudgame_instance "NewEnumerator1")
  (Creation|PrepareLobby)
  (Creation|PreparePlayerList)
  (Creation|PrepareTurnCounter)
  (Assign|AssignCurrentPlayerList)
  (Assign|AssignLobby))

(event Custom|QuitCallback
  ;[1 1 1] All callbacks from Game UI elements are required to go through here
  (bind _asbp_uudgame_instance (Utilities|GetGameInstance))
  (Default|LeaveGame _asbp_uudgame_instance))

(event Custom|StartCallback
  ;[1 1 1] All callbacks from Game UI elements are required to go through here
  (bind _asbp_uudgame_instance (Utilities|GetGameInstance))
  (Default|StartGame _asbp_uudgame_instance))

(event Custom|DisplayTurnCallback
  ;[1 1 1] All callbacks from Game UI elements are required to go through here
  (Assign|AssignTurnCounter))

(event Custom|EndTurnCallback
  ;[1 1 1] All callbacks from Game UI elements are required to go through here
  (bind _asbp_udplayer_controller (Utilities|Casting|CastToBP_UDPlayerController (Game|GetPlayerController 0)))
  (Default|RequestEndTurn _asbp_udplayer_controller))

(event Custom|RefreshTurnCallback
  (params (CurrentTurn :type Integer) (CurrentPlayer :type String))
  ;[1 1 1] All callbacks from Game UI elements are required to go through here
  (Updates|UpdateTurnCounter CurrentTurn CurrentPlayer))

(fn ConstructionScript)

(fn PrepareLobby
  (bind _returnvalue (Game|GetGameMode))
  (Utilities|IsValid (Variables|Default|GetLobbyWidget)
    (:Is%20Not%20Valid
      (bind _returnvalue_2 (UserInterface|CreateWidget "/Game/UnrealDiplomacy/UI/WBP_Lobby.WBP_Lobby_C" (Game|GetPlayerController 0)))
      (bind _output_get (Variables|Default|SetLobbyWidget _returnvalue_2))
      (Utilities|IsValid _returnvalue
        (:Is%20Valid
          (if (Ability|HasAuthority _returnvalue)
            (Default|Enable _output_get)))))))

(fn PreparePlayerList
  (Utilities|IsValid (Variables|Default|GetCurrentPlayerListWidget)
    (:Is%20Not%20Valid
      (bind _returnvalue (UserInterface|CreateWidget "/Game/UnrealDiplomacy/UI/WBP_CurrentPlayersList.WBP_CurrentPlayersList_C" (Game|GetPlayerController 0)))
      (Variables|Default|SetCurrentPlayerListWidget _returnvalue))))

(fn UpdatePlayerList
  (params (PlayerStates :type Array%20of%20Player%20State%20Object%20References))
  (bind _currentplayerlistwidget (Variables|Default|GetCurrentPlayerListWidget))
  (Creation|PreparePlayerList)
  (Default|ClearList _currentplayerlistwidget)
  (Default|CreateList _currentplayerlistwidget PlayerStates))

(fn AssignLobby
  (Creation|PrepareLobby)
  (UserInterface|Viewport|AddtoViewport (Variables|Default|GetLobbyWidget) 0))

(fn AssignCurrentPlayerList
  (Creation|PreparePlayerList)
  (UserInterface|Viewport|AddtoViewport (Variables|Default|GetCurrentPlayerListWidget) 0))

(fn PrepareTurnCounter
  (Utilities|IsValid (Variables|Default|GetTurnCounterWidget)
    (:Is%20Not%20Valid
      (bind _returnvalue (UserInterface|CreateWidget "/Game/UnrealDiplomacy/UI/WBP_TurnCounter.WBP_TurnCounter_C" (Game|GetPlayerController 0)))
      (Variables|Default|SetTurnCounterWidget _returnvalue))))

(fn AssignTurnCounter
  (Creation|PrepareTurnCounter)
  (UserInterface|Viewport|AddtoViewport (Variables|Default|GetTurnCounterWidget) 0))

(fn UpdateTurnCounter
  (params (CurrentTurn :type Integer) (CurrentPlayer :type String))
  (Default|UpdateUI (Variables|Default|GetTurnCounterWidget) CurrentTurn CurrentPlayer))

(fn HideLobby
  (Widget|RemovefromParent (Variables|Default|GetLobbyWidget)))