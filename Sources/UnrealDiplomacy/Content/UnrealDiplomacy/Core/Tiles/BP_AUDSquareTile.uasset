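; BP_AUDSquareTile is a square map tile actor for UnrealDiplomacy that shows ownership and selection state.
; When the owner changes, it hides the flag for Gaia-owned tiles, shows it otherwise, and tints it through the "Banner Color" material parameter, which relies on that exact name.
; Clicks notify tile selection, and select or deselect events toggle the highlight.
; Update and BeginPlay are empty.
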(event EventBeginPlay)

(event EventOnDeselected
  (Rendering|SetVisibility (Variables|Default|GetSelectionHighlight) false true))

(event EventOnSelected
  (Rendering|SetVisibility (Variables|Default|GetSelectionHighlight) true true))

(event MouseInput|EventActorOnClicked
  (params (ButtonPressed :type Key%20Structure :default "None"))
  (Class|UDSquareTile|NotifyTileSelected))

(event EventOnUpdate)

(event EventOnOwnerChanged
  (bind _ownerflag (Variables|Default|GetOwnerFlag))
  ;[1 1 1] This is dependent on name of material !
  (Utilities|FlowControl|Sequence
    (:then_0
      (if (== (Variables|Default|GetTileOwner) (Class|UDGlobalData|GetGaiaFactionId))
        (Rendering|SetVisibility _ownerflag false true)
        (else
          (Rendering|SetVisibility _ownerflag true true))))
    (:then_1
      (Rendering|Material|SetVectorParameterValueonMaterials _ownerflag "Banner Color" (Math|Conversions|ToVector(LinearColor) (Variables|Default|GetOwnerColor))))))

(fn ConstructionScript)