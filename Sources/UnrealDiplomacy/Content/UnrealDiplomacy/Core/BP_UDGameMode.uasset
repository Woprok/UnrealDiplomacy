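; UnrealDiplomacy game mode that runs match setup, player registration and game start.
; On BeginPlay it spawns game, lobby, hex map and turn managers; PostLogin assigns sequential IDs, registering lobby joiners as players (first becomes owner) and later joiners as spectators.
; Server events write settings to the game state; StartGame generates the map from lobby settings.
; Turn and game manager initialization is disconnected; surrender, leave and disconnect handling are unfinished.
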(event EventBeginPlay
  (CallFunction|LogInfo "GameModeBeginPlay" false)
  ;[1 1 1] Initialize Game Mode and his associated Game State
  (Utilities|FlowControl|Sequence
    (:then_0
      ;;[1 1 1] Everytime Game is loaded, (always with Game Level active) we will update our GameInstance to correct state.
      (bind _asbp_uudgame_instance (CallFunction|GetUDGameInstance))
      (Default|SetApplicationState _asbp_uudgame_instance "NewEnumerator1"))
    (:then_1
      ;;[1 1 1] Initialize Game State
      (Initialization|InitializeManagers)
      (Initialization|InitializeManagersDefaults))))

(event EventPostLogin
  (params (NewPlayer :type Player%20Controller%20Object%20Reference))
  (CallFunction|LogInfo "GameModeOnPostLogin" false)
  ;[1 1 1] Each player that joins will be assigned Id from 0 to INT32.MAX
  (bind _asbp_udplayer_controller (Utilities|Casting|CastToBP_UDPlayerController NewPlayer))
  (bind _new_player_id (Initialization|AssignUniqueId _asbp_udplayer_controller))
  ;[1 1 1] Create Player Data that will be saved in Game State for everyone to read access.
  (bind _asbp_udgame_state (CallFunction|GetUDGameState))
  (Utilities|IsinLobby
    (:True
      (Default|CreateNewPlayer _asbp_udgame_state _new_player_id)
      (Initialization|AssignGameOwner _new_player_id))
    (:False
      (Default|CreateNewSpectator _asbp_udgame_state _new_player_id))))

(event EventOnLogout
  (params (ExitingController :type Controller%20Object%20Reference))
  ;[1 1 1] TODO: Allow players to claim nation of player that left (useful for reconnect) + HANDLE DISCONNECT
  (bind _asbp_udplayer_controller (Utilities|Casting|CastToBP_UDPlayerController ExitingController))
  (CallFunction|LogInfo (Utilities|String|ToString(Integer) (Variables|/Game/UnrealDiplomacy/Core/BP_UDPlayerController.BP_UDPlayerController_C|GetAssignedUniqueId _asbp_udplayer_controller)) true))

(event Custom|SurrenderGame
  ;[1 1 1] Comment
)

(event Custom|StartGame
  ;[1 1 1] Comment
  (CallFunction|CreateStart)
  (bind _asbp_udgame_state (CallFunction|GetUDGameState))
  (Variables|/Game/UnrealDiplomacy/Core/BP_UDGameState.BP_UDGameState_C|SetCurrentGameState _asbp_udgame_state "NewEnumerator1"))

(event Custom|LeaveGame
  ;[1 1 1] Comment
)

(event Custom|UpdateLobbySettings
  (params (CurrentGameLobby :type FUD%20Lobby%20Settings%20Structure))
  ;[1 1 1] Comment
  (bind _asbp_udgame_state (CallFunction|GetUDGameState))
  (Variables|/Game/UnrealDiplomacy/Core/BP_UDGameState.BP_UDGameState_C|SetCurrentGameLobby _asbp_udgame_state CurrentGameLobby))

(event Custom|UpdatePlayerSettings
  (params (Owner :type Integer) (NewNationSettngs :type FUD%20Nation%20Settings%20Structure))
  ;[1 1 1] Comment
  (bind _asbp_udgame_state (CallFunction|GetUDGameState))
  (Default|UpdatePlayerSettings _asbp_udgame_state Owner NewNationSettngs))

(fn ConstructionScript
  ;[1 1 1] Initialize Game Mode State (this is not necessary to do (var defaults), but its done for clarity)
  (CallFunction|LogInfo "GameModeConstruct" false)
  (Variables|GameControl|SetNextPlayerUniqueId -1))

(fn InitializeManagers
  (bind _returnvalue (Math|Conversions|ToTransform(Vector) "0, 0,20.000000"))
  (bind _self self)
  (Utilities|FlowControl|Sequence
    (:then_0
      (bind _returnvalue_2 (Game|SpawnActorfromClass "/Game/UnrealDiplomacy/Core/Managers/BP_AUDGameManager.BP_AUDGameManager_C" _returnvalue "Undefined" _self 0))
      (Variables|Managers|SetCurrentGameManager _returnvalue_2))
    (:then_1
      (bind _returnvalue_3 (Game|SpawnActorfromClass "/Game/UnrealDiplomacy/Core/Managers/BP_AUDLobbyManager.BP_AUDLobbyManager_C" _returnvalue "Undefined" _self 0))
      (Variables|Managers|SetCurrentLobbyManager _returnvalue_3))
    (:then_2
      (bind _returnvalue_4 (Game|SpawnActorfromClass "/Game/UnrealDiplomacy/Core/Managers/BP_AUDHexTileGridManager.BP_AUDHexTileGridManager_C" _returnvalue "Undefined" _self 0))
      (Variables|Managers|SetCurrentMapManager _returnvalue_4))
    (:then_3
      (bind _returnvalue_5 (Game|SpawnActorfromClass "/Game/UnrealDiplomacy/Core/Managers/BP_AUDTurnManager.BP_AUDTurnManager_C" _returnvalue "Undefined" _self 0))
      (Variables|Managers|SetCurrentTurnManager _returnvalue_5))
    (:then_4
      (return))))

(fn InitializeManagersDefaults
  (Utilities|FlowControl|Sequence
    (:then_1
      (return))))

(fn AssignGameOwner
  (params (PlayerUniqueId :type Integer))
  (bind _asbp_udgame_state (CallFunction|GetUDGameState))
  (if (== (Variables|/Game/UnrealDiplomacy/Core/BP_UDGameState.BP_UDGameState_C|GetCurrentGameOwner _asbp_udgame_state) -1)
    (Variables|/Game/UnrealDiplomacy/Core/BP_UDGameState.BP_UDGameState_C|SetCurrentGameOwner _asbp_udgame_state PlayerUniqueId))
  (return))

(fn AssignUniqueId
  (params (New%20Player :type BP%20UD%20Player%20Controller%20Object%20Reference))
  ;[1 1 1] Assign unique ID to player for future identification. Starts at -1, so first is always 0.
  (bind _result (Math|Integer|IncrementInt (Variables|GameControl|GetNextPlayerUniqueId))
    (:%20%20
      (bind _output_get (Variables|/Game/UnrealDiplomacy/Core/BP_UDPlayerController.BP_UDPlayerController_C|SetAssignedUniqueId New%20Player _result))
      (return _output_get))))

(fn CreateStart
  (bind _currentmapmanager (Variables|Managers|GetCurrentMapManager))
  (bind _asbp_udgame_state (CallFunction|GetUDGameState))
  (if (Utilities|Enum|Equal(Enum) (Variables|/Game/UnrealDiplomacy/Core/BP_UDGameState.BP_UDGameState_C|GetCurrentGameState _asbp_udgame_state) "NewEnumerator0")
    (Utilities|FlowControl|Sequence
      (:then_0
        ;[1 1 1] Spawn map
        (bind _asbp_udgame_state_2 (CallFunction|GetUDGameState))
        (Utilities|FlowControl|Sequence
          (:then_0
            (Variables|/Script/UnrealDiplomacy.UDHexTileGridManager|SetMapSeed _currentmapmanager (.Seed (Utilities|Struct|BreakFUDLobbySettings (Variables|/Game/UnrealDiplomacy/Core/BP_UDGameState.BP_UDGameState_C|GetCurrentGameLobby _asbp_udgame_state_2)))))
          (:then_1
            (Variables|/Script/UnrealDiplomacy.UDHexTileGridManager|SetGridWidth _currentmapmanager (.Width (Utilities|Struct|BreakFUDLobbySettings (Variables|/Game/UnrealDiplomacy/Core/BP_UDGameState.BP_UDGameState_C|GetCurrentGameLobby _asbp_udgame_state_2)))))
          (:then_2
            (Variables|/Script/UnrealDiplomacy.UDHexTileGridManager|SetGridHeight _currentmapmanager (.Height (Utilities|Struct|BreakFUDLobbySettings (Variables|/Game/UnrealDiplomacy/Core/BP_UDGameState.BP_UDGameState_C|GetCurrentGameLobby _asbp_udgame_state_2)))))
          (:then_3
            (Class|UDHexTileGridManager|Generate _currentmapmanager)
            (return))))
      (:then_2
        (return)))))