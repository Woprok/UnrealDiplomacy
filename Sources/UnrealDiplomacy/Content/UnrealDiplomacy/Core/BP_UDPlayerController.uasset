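; Player controller for UnrealDiplomacy that links each client's HUD and input with the game state.
; Server events forward start, surrender, leave and lobby setting changes to the game state, while end turn is still a stub.
; Client events push match and lobby updates to the HUD, using the assigned unique ID for ownership and player nation.
; Tile clicks are handled locally, opening tile management and switching the selected tile.
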(event EventBeginPlay
  ;[1 1 1] Update settings of this player controller to default required by our game.
  (CallFunction|LogInfo "PlayerControllerBeginPlay" false)
  (CallFunction|SetPlayerControl self))

(event Custom|ServerStartGame
  ;[1 1 1] Provides calls that GameInstance needs to invoke on the Server such as Start, Surrender and Leave Game.
  (bind _asbp_udgame_state (CallFunction|GetUDGameState))
  (Default|OnServerStartGame _asbp_udgame_state))

(event Custom|ServerUpdateLobbySettings
  (params (NewSettings :type FUD%20Lobby%20Settings%20Structure))
  ;[1 1 1] Represents calls that client needs to execute on server like actions. Actions can be for example End Turn, Build, Diplomacy etc.
  (bind _asbp_udgame_state (CallFunction|GetUDGameState))
  (Default|OnServerUpdateLobbySettings _asbp_udgame_state NewSettings))

(event Custom|ServerRequestEndTurn
  ;[1 1 1] Represents calls that client needs to execute on server like actions. Actions can be for example End Turn, Build, Diplomacy etc.
  (CallFunction|GetUDGameState))

(event Custom|ServerLeaveGame
  ;[1 1 1] Provides calls that GameInstance needs to invoke on the Server such as Start, Surrender and Leave Game.
  (bind _asbp_udgame_state (CallFunction|GetUDGameState))
  (Default|OnServerLeaveGame _asbp_udgame_state))

(event Custom|ServerUpdateLobbyPlayerSettings
  (params (NewNationSettings :type FUD%20Nation%20Settings%20Structure))
  ;[1 1 1] Represents calls that client needs to execute on server like actions. Actions can be for example End Turn, Build, Diplomacy etc.
  (bind _asbp_udgame_state (CallFunction|GetUDGameState))
  (Default|OnServerUpdatePlayerSettings _asbp_udgame_state (Variables|Default|GetAssignedUniqueId) NewNationSettings))

(event Custom|ServerSurrenderGame
  ;[1 1 1] Provides calls that GameInstance needs to invoke on the Server such as Start, Surrender and Leave Game.
  (bind _asbp_udgame_state (CallFunction|GetUDGameState))
  (Default|OnServerSurrenderGame _asbp_udgame_state))

(event Custom|OnClientUpdateLobbyPlayerSettings
  (params (Members :type Array%20of%20FUD%20Player%20Data%20Structures))
  ;[1 1 1] Provides events that are used to notify this player controller that some data have changed and this instance should update this client.
  (bind _array_element (Utilities|Array|ForEachLoopwithBreak Members :!label _label)
    (:LoopBody
      (if (== (.UniqueId (Utilities|Struct|BreakFUDPlayerData _array_element)) (Variables|Default|GetAssignedUniqueId))
        (goto _label Break)))
    (:Completed
      (bind _asbp_udhud (CallFunction|GetUDHUD))
      (Default|OnUpdateLobbyPlayerSettings _asbp_udhud (.Nation (Utilities|Struct|BreakFUDPlayerData _array_element))))))

(event Custom|OnClientUpdateLobbySettings
  (params (Owner :type Integer) (LobbyData :type FUD%20Lobby%20Settings%20Structure))
  ;[1 1 1] Provides events that are used to notify this player controller that some data have changed and this instance should update this client.
  (bind _asbp_udhud (CallFunction|GetUDHUD))
  (Default|OnUpdateLobbySettings _asbp_udhud Owner LobbyData (CallFunction|IsOwner Owner)))

(event Custom|OnClientUpdateLobbyMembers
  (params (Members :type Array%20of%20FUD%20Player%20Data%20Structures))
  ;[1 1 1] Provides events that are used to notify this player controller that some data have changed and this instance should update this client.
  (bind _asbp_udhud (CallFunction|GetUDHUD))
  (Default|OnUpdateLobbyMembers _asbp_udhud Members))

(event Custom|OnClientUpdateMatchStateUI
  (params (MatchUI :type EUDMatchState%20Enum :default "NewEnumerator0"))
  ;[1 1 1] Provides events that are used to notify this player controller that some data have changed and this instance should update this client.
  (bind _asbp_udhud (CallFunction|GetUDHUD))
  (Default|OnUpdateMatchStateUI _asbp_udhud MatchUI))

(event Custom|OnTileClicked
  (params (Tile :type BP%20AUD%20Hex%20Tile%20Object%20Reference))
  (bind _returnvalue (Utilities|GetDisplayName Tile))
  ;[1 1 1] Comment
  (Utilities|FlowControl|Sequence
    (:then_0
      (bind _asbp_udhud (CallFunction|GetUDHUD))
      (Default|ShowTileManegement _asbp_udhud (Utilities|String|Append _returnvalue " at " (Utilities|String|ToString(Integer) (Variables|/Script/UnrealDiplomacy.UDHexTile|GetTileIndex (Variables|Default|GetSelectedTile))))))
    (:then_1
      (Default|OnDeselected (Variables|Default|GetSelectedTile)))
    (:then_2
      (bind _output_get (Variables|Default|SetSelectedTile Tile))
      (Default|OnSelected _output_get))
    (:then_3
      (CallFunction|LogInfo (Utilities|String|Append "Selected Tile " _returnvalue) true))))

(fn ConstructionScript
  (CallFunction|LogInfo "PlayerControllerConstruct" false))

(fn IsOwner
  (params (OwnerId :type Integer))
  (return (== OwnerId (Variables|Default|GetAssignedUniqueId))))