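; BP_Helpers is a Blueprint helper library of shared utilities for UnrealDiplomacy's main menu and skirmish modes.
; Typed getters cast the game instance, game mode, game state, and first player's controller and HUD to project classes.
; Color-coded log functions print messages, and a failed game mode cast logs an unauthorized client access error.
; Settings functions sync screen mode and resolution combo boxes with GameUserSettings, applying them on save.
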(fn LogError
  (params (Message :type String) (bPrintToScreen :type Boolean))
  (Development|PrintString (LocalVariables|Get__WorldContext) Message bPrintToScreen true "(R=1.000000,G=0.000000,B=0.000000,A=1.000000)" 6e+01)
  (return))

(fn LogInfo
  (params (Message :type String) (bPrintToScreen :type Boolean))
  (Development|PrintString (LocalVariables|Get__WorldContext) Message bPrintToScreen true "(R=0.000000,G=1.000000,B=0.000000,A=1.000000)" 6e+01)
  (return))

(fn LogWarning
  (params (Message :type String) (bPrintToScreen :type Boolean))
  (Development|PrintString (LocalVariables|Get__WorldContext) Message bPrintToScreen true "(R=1.000000,G=1.000000,B=0.000000,A=1.000000)" 6e+01)
  (return))

(fn GetUDGameInstance
  (bind _asbp_udgame_instance (Utilities|Casting|CastToBP_UDGameInstance (Game|GetGameInstance (LocalVariables|Get__WorldContext))))
  (return _asbp_udgame_instance))

(fn GetMainMenuUDHUD
  (bind _asbp_main_menu_udhud (Utilities|Casting|CastToBP_MainMenuUDHUD (HUD|GetHUD (Game|GetPlayerController (LocalVariables|Get__WorldContext)))))
  (return _asbp_main_menu_udhud))

(fn GetUDHUD
  (bind _asbp_udskirmish_hud (Utilities|Casting|CastToBP_UDSkirmishHUD (HUD|GetHUD (Game|GetPlayerController (LocalVariables|Get__WorldContext)))))
  (return _asbp_udskirmish_hud))

(fn LoadSettings
  (params (ScreenMode :type Combo%20Box%20String%20Object%20Reference) (Resolution :type Combo%20Box%20String%20Object%20Reference))
  (bind _returnvalue (Settings|GetGameUserSettings))
  (Utilities|FlowControl|Sequence
    (:then_0
      ;[1 1 1] Setup ComboBox
      (bind _enumvalue (|ForEachEWindowMode)
        (:LoopBody
          (Class|ComboBoxString|AddOption ScreenMode (Utilities|String|EnumtoString _enumvalue)))))
    (:then_1
      ;[1 1 1] Set ScreenMode
      (Class|ComboBoxString|SetSelectedOption ScreenMode (Utilities|String|EnumtoString (Class|GameUserSettings|GetFullscreenMode _returnvalue))))
    (:then_2
      ;[1 1 1] Set Resolution
      (Class|ComboBoxString|SetSelectedOption Resolution (Utilities|String|Append (Utilities|String|ToString(Integer) (Class|KismetMathLibrary|FTrunc64 (.X (Math|Vector2D|BreakVector2D (Math|Conversions|ToVector2D(IntPoint) (Class|GameUserSettings|GetScreenResolution _returnvalue)))))) "x" (Utilities|String|ToString(Integer) (Class|KismetMathLibrary|FTrunc64 (.Y (Math|Vector2D|BreakVector2D (Math|Conversions|ToVector2D(IntPoint) (Class|GameUserSettings|GetScreenResolution _returnvalue)))))))))
    (:then_3
      (return))))

(fn SaveSettings
  (params (ScreenMode :type Combo%20Box%20String%20Object%20Reference) (Resolution :type Combo%20Box%20String%20Object%20Reference))
  (bind _returnvalue (Class|ComboBoxString|GetSelectedOption Resolution))
  (bind (_lefts _rights) (Utilities|String|Split _returnvalue "x"))
  (bind _returnvalue_2 (Settings|GetGameUserSettings))
  (Utilities|FlowControl|Sequence
    (:then_0
      ;[1 1 1] Set Resolution
      (Class|GameUserSettings|SetScreenResolution _returnvalue_2 (Utilities|Struct|MakeIntPoint (Math|Conversions|ToInteger(Byte) _lefts) (Math|Conversions|ToInteger(Byte) _rights))))
    (:then_1
      ;[1 1 1] Set ScreenMode
      (Class|GameUserSettings|SetFullscreenMode _returnvalue_2 (Utilities|Enum|ByteToEnumEWindowMode (Math|Conversions|ToByte(Integer) (Class|ComboBoxString|GetSelectedIndex ScreenMode)))))
    (:then_2
      ;[1 1 1] Apply Resolution
      (Class|GameUserSettings|ApplyResolutionSettings _returnvalue_2 false))
    (:then_3
      ;[1 1 1] Apply Settings
      (Class|GameUserSettings|ApplySettings _returnvalue_2 false))
    (:then_4
      (return))))

(fn GetUDGameState
  (bind _asbp_udskirmish_game_state (Utilities|Casting|CastToBP_UDSkirmishGameState (Game|GetGameState (LocalVariables|Get__WorldContext))))
  (return _asbp_udskirmish_game_state))

(fn GetUDPlayerController
  (bind _asbp_udskirmish_player_controller (Utilities|Casting|CastToBP_UDSkirmishPlayerController (Game|GetPlayerController (LocalVariables|Get__WorldContext))))
  (return _asbp_udskirmish_player_controller))

(fn GetUDGameMode
  (bind ___worldcontext (LocalVariables|Get__WorldContext))
  (bind _asbp_udskirmish_game_mode (Utilities|Casting|CastToBP_UDSkirmishGameMode (Game|GetGameMode ___worldcontext))
    (:then
      (return _asbp_udskirmish_game_mode))
    (:CastFailed
      (Debug|LogError "UNAUTHORIZED ACCESS TO GAMEMODE ON CLIENT" true ___worldcontext))))

(fn GetMainMenuUDPlayerController
  (bind _asbp_main_menu_udplayer_controller (Utilities|Casting|CastToBP_MainMenuUDPlayerController (Game|GetPlayerController (LocalVariables|Get__WorldContext))))
  (return _asbp_main_menu_udplayer_controller))