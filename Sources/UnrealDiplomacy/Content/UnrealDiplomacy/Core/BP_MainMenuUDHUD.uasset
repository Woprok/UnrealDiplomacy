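; Main menu HUD for UnrealDiplomacy that switches between main, join game, options and credits screens and handles all their button callbacks.
; Each screen widget is created lazily, cached, and shown alone after clearing the others.
; Host, join, search, tutorial and quit go to the game instance, whose session-search events fill the join list, prepared at BeginPlay.
; It also loads and saves screen mode and resolution through GameUserSettings.
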(event Custom|OnValidSessionList
  (params (Sessions :type Array%20of%20Blueprint%20Session%20Result%20Structures))
  ;[1 1 1] Initialization
  ;;[1 1 1] Initialize Join Game
  (Default|SetList (Variables|Widgets|GetJoinGameMenuWidget) Sessions))

(event Custom|OnEmptySessionList
  ;[1 1 1] Initialization
  ;;[1 1 1] Initialize Join Game
  (Default|SetNoList (Variables|Widgets|GetJoinGameMenuWidget)))

(event EventBeginPlay
  ;[1 1 1] Initialization
  (Utilities|FlowControl|Sequence
    (:then_0
      ;;[1 1 1] Initialize Join Game
      (Widgets|PrepareJoinGameMenu)
      (bind _asbp_uudgame_instance (Utilities|GetGameInstance))
      (EventDispatchers|BindEventtoOnValidSessionList _asbp_uudgame_instance (delegate Custom|OnValidSessionList))
      (EventDispatchers|BindEventtoOnEmptySessionList _asbp_uudgame_instance (delegate Custom|OnEmptySessionList)))
    (:then_1
      ;;[1 1 1] Progress to initial UI
      (Widgets|SwitchtoMainMenu))))

(event Custom|InvokeOnBackClicked
  ;[1 1 1] All callbacks from Menu UI elements are required to go through here
  (Widgets|SwitchtoMainMenu))

(event Custom|InvokeOnOptionsClicked
  ;[1 1 1] All callbacks from Menu UI elements are required to go through here
  (Widgets|SwitchtoOptionsMenu))

(event Custom|InvokeOnHostClicked
  ;[1 1 1] All callbacks from Menu UI elements are required to go through here
  (bind _asbp_uudgame_instance (Utilities|GetGameInstance))
  (Default|CreateGame _asbp_uudgame_instance))

(event Custom|InvokeOnSaveSettingsClicked
  (params (ScreenMode :type Combo%20Box%20String%20Object%20Reference) (Resolution :type Combo%20Box%20String%20Object%20Reference))
  ;[1 1 1] All callbacks from Menu UI elements are required to go through here
  (Settings|SaveSettings ScreenMode Resolution))

(event Custom|InvokeOnJoinClicked
  ;[1 1 1] All callbacks from Menu UI elements are required to go through here
  (Widgets|SwitchtoJoinGameMenu))

(event Custom|InvokeOnTutorialClicked
  ;[1 1 1] All callbacks from Menu UI elements are required to go through here
  (bind _asbp_uudgame_instance (Utilities|GetGameInstance))
  (Default|CreateTutorialGame _asbp_uudgame_instance))

(event Custom|InvokeOnQuitClicked
  ;[1 1 1] All callbacks from Menu UI elements are required to go through here
  (bind _asbp_uudgame_instance (Utilities|GetGameInstance))
  (Default|QuitfromMainMenu _asbp_uudgame_instance))

(event Custom|InvokeOnSearchForGamesClicked
  ;[1 1 1] All callbacks from Menu UI elements are required to go through here
  (bind _asbp_uudgame_instance (Utilities|GetGameInstance))
  (Default|SearchforGames _asbp_uudgame_instance))

(event Custom|InvokeOnCreditsClicked
  ;[1 1 1] All callbacks from Menu UI elements are required to go through here
  (Widgets|SwitchtoCreditsMenu))

(event Custom|InvokeOnJoinGameClicked
  (params (SearchResult :type Blueprint%20Session%20Result%20Structure%20%28by%20ref%29))
  ;[1 1 1] All callbacks from Menu UI elements are required to go through here
  (bind _asbp_uudgame_instance (Utilities|GetGameInstance))
  (Default|JoinGame _asbp_uudgame_instance SearchResult))

(fn ConstructionScript)

(fn PrepareJoinGameMenu
  (Utilities|IsValid (Variables|Widgets|GetJoinGameMenuWidget)
    (:Is%20Not%20Valid
      (bind _returnvalue (UserInterface|CreateWidget "/Game/UnrealDiplomacy/UI/Menu/WBP_JoinGameMenu.WBP_JoinGameMenu_C" (Game|GetPlayerController 0)))
      (Variables|Widgets|SetJoinGameMenuWidget _returnvalue))))

(fn PrepareCreditsMenu
  (Utilities|IsValid (Variables|Widgets|GetCreditsMenuWidget)
    (:Is%20Not%20Valid
      (bind _returnvalue (UserInterface|CreateWidget "/Game/UnrealDiplomacy/UI/Menu/WBP_CreditsMenu.WBP_CreditsMenu_C" (Game|GetPlayerController 0)))
      (Variables|Widgets|SetCreditsMenuWidget _returnvalue))))

(fn PrepareMainMenu
  (Utilities|IsValid (Variables|Widgets|GetMainMenuWidget)
    (:Is%20Not%20Valid
      (bind _returnvalue (UserInterface|CreateWidget "/Game/UnrealDiplomacy/UI/Menu/WBP_MainMenu.WBP_MainMenu_C" (Game|GetPlayerController 0)))
      (Variables|Widgets|SetMainMenuWidget _returnvalue))))

(fn PrepareOptionsMenu
  (Utilities|IsValid (Variables|Widgets|GetOptionsMenuWidget)
    (:Is%20Not%20Valid
      (bind _returnvalue (UserInterface|CreateWidget "/Game/UnrealDiplomacy/UI/Menu/WBP_OptionsMenu.WBP_OptionsMenu_C" (Game|GetPlayerController 0)))
      (Variables|Widgets|SetOptionsMenuWidget _returnvalue))))

(fn SwitchtoJoinGameMenu
  (Viewport|RemoveAllWidgets)
  (Widgets|PrepareJoinGameMenu)
  (UserInterface|Viewport|AddtoViewport (Variables|Widgets|GetJoinGameMenuWidget) 0))

(fn SwitchtoOptionsMenu
  (Viewport|RemoveAllWidgets)
  (Widgets|PrepareOptionsMenu)
  (UserInterface|Viewport|AddtoViewport (Variables|Widgets|GetOptionsMenuWidget) 0))

(fn SwitchtoMainMenu
  (Viewport|RemoveAllWidgets)
  (Widgets|PrepareMainMenu)
  (UserInterface|Viewport|AddtoViewport (Variables|Widgets|GetMainMenuWidget) 0))

(fn SwitchtoCreditsMenu
  (Viewport|RemoveAllWidgets)
  (Widgets|PrepareCreditsMenu)
  (UserInterface|Viewport|AddtoViewport (Variables|Widgets|GetCreditsMenuWidget) 0))

(fn LoadSettings
  (params (ScreenMode :type Combo%20Box%20String%20Object%20Reference) (Resolution :type Combo%20Box%20String%20Object%20Reference))
  (bind _enumvalue (|ForEachEWindowMode)
    (:LoopBody
      (Class|ComboBoxString|AddOption ScreenMode (Utilities|String|EnumtoString _enumvalue))
      (bind _returnvalue (Settings|GetGameUserSettings))
      (Class|ComboBoxString|SetSelectedOption ScreenMode (Utilities|String|EnumtoString (Class|GameUserSettings|GetFullscreenMode _returnvalue)))
      (Class|ComboBoxString|SetSelectedOption Resolution (Utilities|String|Append (Utilities|String|ToString(Integer) (Class|KismetMathLibrary|FTrunc64 (.X (Math|Vector2D|BreakVector2D (Math|Conversions|ToVector2D(IntPoint) (Class|GameUserSettings|GetScreenResolution _returnvalue)))))) "x" (Utilities|String|ToString(Integer) (Class|KismetMathLibrary|FTrunc64 (.Y (Math|Vector2D|BreakVector2D (Math|Conversions|ToVector2D(IntPoint) (Class|GameUserSettings|GetScreenResolution _returnvalue)))))))))))

(fn SaveSettings
  (params (ScreenMode :type Combo%20Box%20String%20Object%20Reference) (Resolution :type Combo%20Box%20String%20Object%20Reference))
  (bind _returnvalue (Class|ComboBoxString|GetSelectedOption Resolution))
  (bind (_lefts _rights) (Utilities|String|Split _returnvalue "x"))
  (bind _returnvalue_2 (Settings|GetGameUserSettings))
  (Class|GameUserSettings|SetScreenResolution _returnvalue_2 (Utilities|Struct|MakeIntPoint (Math|Conversions|ToInteger(Byte) _lefts) (Math|Conversions|ToInteger(Byte) _rights)))
  (Class|GameUserSettings|SetFullscreenMode _returnvalue_2 (Utilities|Enum|ByteToEnumEWindowMode (Math|Conversions|ToByte(Integer) (Class|ComboBoxString|GetSelectedIndex ScreenMode))))
  (Class|GameUserSettings|ApplyResolutionSettings _returnvalue_2 false)
  (Class|GameUserSettings|ApplySettings _returnvalue_2 false))