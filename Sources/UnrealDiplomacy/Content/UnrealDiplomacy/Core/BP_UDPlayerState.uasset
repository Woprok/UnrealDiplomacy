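; BP_UDPlayerState is the Unreal Diplomacy player state, holding a player's Resources and keeping them in sync with game data.
; On BeginPlay it calls OnCurrentPlayerFinilized on BP_UDGameState.
; A replicated IsDirty flag marks stale data: its OnRep re-reads Resources from the game state's CurrentGameManager by JoinId, clears the flag and refreshes the HUD's player information bar.
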(event Custom|UpdateHUD
  (bind _asbp_udhud (Utilities|Casting|CastToBP_UDHUD (HUD|GetHUD (Game|GetPlayerController 0))))
  (Default|UpdatePlayerInformationBar _asbp_udhud))

(event EventBeginPlay
  (bind _asbp_udgame_state (Utilities|Casting|CastToBP_UDGameState (Game|GetGameState)))
  (Default|OnCurrentPlayerFinilized _asbp_udgame_state))

(fn ConstructionScript)

(fn OnRepIsDirty
  ;[1 1 1] If something is IsDirty it means that it contains incorrect data
  (if (Variables|Default|GetIsDirty)
    (bind _asbp_udgame_state (Utilities|Casting|CastToBP_UDGameState (Game|GetGameState)))
    (bind _mydata (Default|GetPlayerData (Variables|/Game/UnrealDiplomacy/Core/BP_UDGameState.BP_UDGameState_C|GetCurrentGameManager _asbp_udgame_state) (Variables|Default|GetJoinId)))
    (Variables|Default|SetResources (.Resources (Utilities|Struct|BreakPlayerData _mydata)))
    (Variables|Default|SetIsDirty false)
    (CallFunction|UpdateHUD)))