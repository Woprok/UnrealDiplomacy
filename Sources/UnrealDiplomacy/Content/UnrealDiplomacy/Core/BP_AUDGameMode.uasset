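; Game mode for UnrealDiplomacy that sets up the hex map and registers players as they log in.
; PostLogin triggers a one-time spawn and generation of a fixed-seed hex grid when the game instance state is Standard.
; On authority, it sets each player's join ID from the PlayerArray length, then notifies the game state of the player change.
; An uncalled example function respawns a controller as a spectator pawn at a PlayerStart.
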(event Custom|SpawnMap
  (if (not (Variables|Default|GetIsSpawned))
    (bind _asbp_uudgame_instance (Utilities|Casting|CastToBP_UUDGameInstance (Game|GetGameInstance)))
    (bind _gameinstancestate (Default|GetCurrentGameInstanceState _asbp_uudgame_instance))
    (switch Utilities|FlowControl|Switch|SwitchonEGameInstanceState _gameinstancestate
      (:NewEnumerator1
        (bind _returnvalue (Game|SpawnActorfromClass "/Game/UnrealDiplomacy/HexTiles/BP_AUDHexTileGridManager.BP_AUDHexTileGridManager_C" (Math|Conversions|ToTransform(Vector) "0, 0,20.000000") "Undefined" 0 0))
        (Variables|/Script/UnrealDiplomacy.UDHexTileGridManager|SetMapSeed _returnvalue 671996)
        (Variables|/Script/UnrealDiplomacy.UDHexTileGridManager|SetGridWidth _returnvalue 5)
        (Variables|/Script/UnrealDiplomacy.UDHexTileGridManager|SetGridHeight _returnvalue 5)
        (Variables|Default|SetIsSpawned true)
        (Class|UDHexTileGridManager|Generate _returnvalue)))))

(event EventBeginPlay)

(event EventPostLogin
  (params (NewPlayer :type Player%20Controller%20Object%20Reference))
  (CallFunction|SpawnMap)
  (bind _asbp_audplayer_controller (Utilities|Casting|CastToBP_AUDPlayerController NewPlayer))
  (Utilities|DefinePlayerJoinId _asbp_audplayer_controller
    (:Output
      (Networking|SwitchHasAuthority
        (:Authority
          (bind _asbp_audgame_state (Utilities|Casting|CastToBP_AUDGameState (Game|GetGameState)))
          (Default|OnCurrentPlayersChanged _asbp_audgame_state))
        (:Remote
          (Development|PrintString "Hello"))))))

(event EventTick
  (params (DeltaSeconds :type Float%20%28single-precision%29)))

(fn ConstructionScript)