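; Game instance for UnrealDiplomacy that manages online sessions, level switching and global UI.
; Creates, joins, finds and destroys sessions, opening the game map as a listen server and broadcasting search results; tutorial is a stub.
; Start, leave and surrender requests go to the player controller's server calls.
; Failures are logged or shown in error dialogs layered above a reusable loading screen, and it also tracks application state.
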(event Custom|SearchForGames
  ;[1 1 1] Find games
  (bind _results (|FindSessions (Game|GetPlayerController 0) 20 false)
    (:OnSuccess
      (if (!= (Utilities|Array|Length _results) 0)
        (Variables|Multiplayer|SetHasSessionList true)
        (bind _output_get (Variables|Multiplayer|SetCurrentSessionList _results))
        (Default|CallOnValidSessionList _output_get)
        (else
          (CallFunction|LogError "No Session found." false)
          (Variables|Multiplayer|SetHasSessionList false :!label _label)
          (Default|CallOnEmptySessionList))))
    (:OnFailure
      (CallFunction|LogError "Session search failed." false)
      (goto _label))))

(event Custom|JoinGame
  (params (SearchResult :type Blueprint%20Session%20Result%20Structure%20%28by%20ref%29))
  ;[1 1 1] Join Game
  (|JoinSession (Game|GetPlayerController 0) SearchResult
    (:OnSuccess
      (CallFunction|LogInfo "Joining session." false))
    (:OnFailure
      (Widget|DisplayErrorDialog "JOIN ERROR" "Session is no longer available."))))

(event Custom|CreateGame
  ;[1 1 1] Create Game
  (|Session (Game|GetPlayerController 0) 10 false
    (:OnSuccess
      (CallFunction|MovetoGame))
    (:OnFailure
      (Widget|DisplayErrorDialog "CREATE ERROR" "Session can not be created."))))

(event Custom|SurrenderGame
  ;[1 1 1] Game control events and actions
  (bind _asbp_udplayer_controller (CallFunction|GetUDPlayerController))
  (Default|ServerSurrenderGame _asbp_udplayer_controller))

(event Custom|StartGame
  ;[1 1 1] Game control events and actions
  (bind _asbp_udplayer_controller (CallFunction|GetUDPlayerController))
  (Default|ServerStartGame _asbp_udplayer_controller))

(event Custom|CreateTutorialGame
  ;[1 1 1] Create Tutorial Game
  (Widget|DisplayErrorDialog "NOT IMPLEMENTED" "Tutorial is not part of this version. Please be patient while we craft new experience for you."))

(event Custom|LeaveGame
  ;[1 1 1] Game control events and actions
  (bind _asbp_udplayer_controller (CallFunction|GetUDPlayerController))
  (Utilities|FlowControl|Sequence
    (:then_0
      (Default|ServerLeaveGame _asbp_udplayer_controller))
    (:then_1
      (|DestroySession _asbp_udplayer_controller
        (:OnSuccess
          _)
        (:OnFailure
          (CallFunction|LogError "Session descrution failed." false)))
      (CallFunction|MovetoMainMenu))))

(event EventHandleTravelError
  (params (FailureType :type ETravelFailure%20Enum :default "NoLevel"))
  ;[1 1 1] Error Handling
  (Widget|DisplayErrorDialog "CONNECTION ERROR" (Multiplayer|TravelErrortoString FailureType)))

(event EventHandleNetworkError
  (params (FailureType :type ENetworkFailure%20Enum :default "NetDriverAlreadyExists") (bIsServer :type Boolean))
  (bind _message (Multiplayer|NetErrortoString FailureType))
  ;[1 1 1] Error Handling
  (if bIsServer
    (CallFunction|LogError _message false)
    (else
      (Widget|DisplayErrorDialog "CONNECTION ERROR" _message))))

(event Custom|QuitFromMainMenu
  ;[1 1 1] Switching between different levels/maps.
  (Game|QuitGame 0 "Quit" false))

(event Custom|MoveToGame
  ;[1 1 1] Switching between different levels/maps.
  (Game|OpenLevel(byObjectReference) "/Game/UnrealDiplomacy/Skirmish/Maps/Standard.Standard" true "listen"))

(event Custom|MoveToMainMenu
  ;[1 1 1] Switching between different levels/maps.
  (Game|OpenLevel(byObjectReference) "/Game/UnrealDiplomacy/Menu/Maps/MainMenu.MainMenu"))

(event Custom|InvokeOnOkErrorClicked
  (params (Error%20Widget :type WBP%20Error%20Dialog%20Object%20Reference))
  ;[1 1 1] Special universal UI handles
  (Widget|CloseErrorDialog Error%20Widget))

(fn PrepareLoadingScreen
  (Utilities|IsValid (Variables|Widgets|GetLoadingScreenWidget)
    (:Is%20Valid
      _)
    (:Is%20Not%20Valid
      (bind _returnvalue (UserInterface|CreateWidget "/Game/UnrealDiplomacy/Core/UI/WBP_LoadingScreen.WBP_LoadingScreen_C" (Game|GetPlayerController 0)))
      (Variables|Widgets|SetLoadingScreenWidget _returnvalue)))
  (return (Variables|Widgets|GetLoadingScreenWidget)))

(fn AssignLoadingScreen
  (bind _widget (Widget|PrepareLoadingScreen))
  (UserInterface|Viewport|AddtoViewport _widget 9)
  (return))

(fn CreateErrorDialog
  (bind _returnvalue (UserInterface|CreateWidget "/Game/UnrealDiplomacy/Core/UI/WBP_ErrorDialog.WBP_ErrorDialog_C" (Game|GetPlayerController 0)))
  (return _returnvalue))

(fn AssignErrorDialog
  (bind _errordialog (Widget|CreateErrorDialog))
  (UserInterface|Viewport|AddtoViewport _errordialog 10)
  (return _errordialog))

(fn DisplayErrorDialog
  (params (Title :type String) (Message :type String))
  (bind _errordialog (Widget|AssignErrorDialog))
  (Default|SetContent _errordialog Title Message)
  (return))

(fn CloseErrorDialog
  (params (DialogWidget :type Widget%20Object%20Reference))
  (Widget|RemovefromParent DialogWidget)
  (return))

(fn SetApplicationState
  (params (CurrentState :type EUDApplicationState%20Enum :default "NewEnumerator3"))
  (bind _output_get (Variables|StateManagement|SetCurrentState CurrentState))
  (CallFunction|LogInfo (Utilities|String|Append "Changed state to: " (Utilities|String|EnumtoString _output_get)) false)
  (return _output_get))

(fn TravelErrortoString
  (params (TravelError :type ETravelFailure%20Enum :default "NoLevel"))
  (return (Utilities|String|Append "Error: failed to travel." (Utilities|String|EnumtoString TravelError))))

(fn NetErrortoString
  (params (NetError :type ENetworkFailure%20Enum :default "NetDriverAlreadyExists"))
  (switch Utilities|FlowControl|Switch|SwitchonENetworkFailure NetError
    (:NetDriverAlreadyExists
      (LocalVariables|SetErrorString (Utilities|String|Append "Error: lost connection due to  " (Utilities|String|EnumtoString NetError) ".") :!label _label))
    (:NetDriverCreateFailure
      (goto _label))
    (:NetDriverListenFailure
      (goto _label))
    (:ConnectionLost
      (goto _label))
    (:ConnectionTimeout
      (LocalVariables|SetErrorString "Error: connection timed out."))
    (:FailureReceived
      (goto _label))
    (:OutdatedClient
      (goto _label))
    (:OutdatedServer
      (goto _label))
    (:PendingConnectionFailure
      (goto _label))
    (:NetGuidMismatch
      (LocalVariables|SetErrorString "Error: Checksum or Guid Mismatch." :!label _label_2))
    (:NetChecksumMismatch
      (goto _label_2)))
  (return (LocalVariables|GetErrorString)))

(fn GetApplicationState
  (return (Variables|StateManagement|GetCurrentState)))