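; BP_UDTurnManager tracks the turn count and active player, cycling through the player list in order.
; ServerInitialize sets the first player and shows the turn counter through the HUD.
; End-turn requests advance play only when the requester's ID matches the current player index, then call TurnEnded on the game state's CurrentGameManager.
; RepNotifies on turn and player name refresh player controller 0's HUD.
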(event Custom|OnServerPlayerEndsTurn
  (params (PlayerId :type Integer))
  ;[1 1 1] Server Executed, Player ends turn,for example before game decides to end it for him.
  (CallFunction|MyServerEvent PlayerId))

(event Custom|ServerInitialize
  (params (Players :type Array%20of%20Player%20State%20Object%20References))
  ;[1 1 1] Server Executed
  (Variables|Default|SetCurrentTurn 0)
  (Variables|Default|SetPlayers Players)
  (bind _output_get (Variables|Default|SetCurrentPlayerIndex 0))
  (Variables|Default|SetCurrentPlayer (PlayerState|GetPlayerName (Utilities|Array|Get(acopy) Players _output_get)))
  (CallFunction|ShowTurnCounter))

(event Custom|ShowTurnCounter
  (bind _returnvalue (Game|GetPlayerController 0))
  (Development|PrintString (Utilities|String|Append "PC: " (Utilities|GetDisplayName (Variables|/Script/Engine.Controller|GetPlayerState _returnvalue))))
  (bind _asbp_udhud (Utilities|Casting|CastToBP_UDHUD (HUD|GetHUD _returnvalue)))
  (Default|DisplayTurnCallback _asbp_udhud))

(event Custom|MyServerEvent
  (params (RequestorPlayerID :type Integer))
  (bind _players (Variables|Default|GetPlayers))
  ;[1 1 1] Server Executed, Player ends turn,for example before game decides to end it for him.
  (Networking|SwitchHasAuthority
    (:Authority
      (Development|PrintString "Server requests to end turn."))
    (:Remote
      (Development|PrintString "Client requests to end turn.")))
  (if (== (Variables|Default|GetCurrentPlayerIndex) RequestorPlayerID)
    (Variables|Default|SetCurrentTurn (+ (Variables|Default|GetCurrentTurn) 1))
    (if (< (+ (Variables|Default|GetCurrentPlayerIndex) 1) (Utilities|Array|Length _players))
      (bind _output_get (Variables|Default|SetCurrentPlayerIndex (+ (Variables|Default|GetCurrentPlayerIndex) 1)))
      (Variables|Default|SetCurrentPlayer (PlayerState|GetPlayerName (Utilities|Array|Get(acopy) _players _output_get)))
      (else
        (bind _output_get_2 (Variables|Default|SetCurrentPlayerIndex 0))
        (Variables|Default|SetCurrentPlayer (PlayerState|GetPlayerName (Utilities|Array|Get(acopy) _players _output_get_2)))))
    (bind _asbp_udgame_state (Utilities|Casting|CastToBP_UDGameState (Game|GetGameState)))
    (Default|TurnEnded (Variables|/Game/UnrealDiplomacy/Core/BP_UDGameState.BP_UDGameState_C|GetCurrentGameManager _asbp_udgame_state))
    (else
      (Development|PrintString "Unauthorized end turn requested. Its not your turn."))))

(event Custom|DisplayedDataChanged
  ;[1 1 1] Visual Update
  (bind _asbp_udhud (Utilities|Casting|CastToBP_UDHUD (HUD|GetHUD (Game|GetPlayerController 0))))
  (Default|RefreshTurnCallback _asbp_udhud (Variables|Default|GetCurrentTurn) (Variables|Default|GetCurrentPlayer)))

(fn ConstructionScript)

(fn OnRepCurrentTurn
  (CallFunction|DisplayedDataChanged))

(fn OnRepCurrentPlayer
  (CallFunction|DisplayedDataChanged))

(fn OnRepCurrentPlayerIndex)