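; Game manager for UnrealDiplomacy that sets up the match's players and drives the player information bar.
; ServerInitialize, marked as server-executed, stores the players and walks every DTUDResources row for each player state, but does nothing with the rows yet.
; It then has player controller 0's BP_UDHUD assign the bar.
; DisplayedDataChanged asks that same HUD to refresh it.
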(event Custom|DisplayedDataChanged
  ;[1 1 1] Visual Update
  (bind _asbp_udhud (Utilities|Casting|CastToBP_UDHUD (HUD|GetHUD (Game|GetPlayerController 0))))
  (Default|UpdatePlayerInformationBar _asbp_udhud))

(event Custom|ServerInitialize
  (params (Players :type Array%20of%20Player%20State%20Object%20References))
  ;[1 1 1] Server Executed
  (bind _output_get (Variables|Default|SetPlayers Players))
  (for _array_element _output_get
    (Utilities|Casting|CastToBP_UDPlayerState _array_element)
    (bind _outrownames (DataTable|GetDataTableRowNames "/Game/UnrealDiplomacy/Data/DTUDResources.DTUDResources"))
    (for _array_element_2 _outrownames
      (Utilities|GetDataTableRow "/Game/UnrealDiplomacy/Data/DTUDResources.DTUDResources" _array_element_2)))
  (CallFunction|ShowPlayerInfoBar))

(event Custom|ShowPlayerInfoBar
  (bind _asbp_udhud (Utilities|Casting|CastToBP_UDHUD (HUD|GetHUD (Game|GetPlayerController 0))))
  (Default|AssignPlayerInformationBar _asbp_udhud))

(fn ConstructionScript)