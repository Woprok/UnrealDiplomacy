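; Game manager for UnrealDiplomacy that stores the player list and per-player resource data built from the DTUDResources data table.
; ServerInitialize stores players, logs the local PlayerState and toggles IsDirty, a RepNotify meant to trigger visual updates through DisplayedDataChanged.
; GetPlayerData looks up records by join ID, returning a placeholder when missing.
; It is unfinished: HUD update and TurnEnded only cast, while player-data creation and resource-change test are unwired.
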(event Custom|DisplayedDataChanged
  ;[1 1 1] Visual Update
  (Utilities|Casting|CastToBP_UDHUD (HUD|GetHUD (Game|GetPlayerController 0))))

(event Custom|ServerInitialize
  (params (Players :type Array%20of%20Player%20State%20Object%20References))
  ;[1 1 1] Server Executed
  (bind _output_get (Variables|Default|SetPlayers Players))
  (for _array_element _output_get
    (Utilities|Casting|CastToBP_UDPlayerState _array_element))
  (CallFunction|ShowPlayerInfoBar)
  (Variables|Default|SetIsDirty true)
  (Variables|Default|SetIsDirty false))

(event Custom|ShowPlayerInfoBar
  (bind _returnvalue (Game|GetPlayerController 0))
  (CallFunction|LogInfo (Utilities|String|Append "PC: " (Utilities|GetDisplayName (Variables|/Script/Engine.Controller|GetPlayerState _returnvalue))) true)
  (Utilities|Casting|CastToBP_UDHUD (HUD|GetHUD _returnvalue)))

(event Custom|TurnEnded
  ;[1 1 1] Test Of Resource Change
  (for _array_element (Variables|Default|GetPlayers)
    (bind _asbp_udplayer_state (Utilities|Casting|CastToBP_UDPlayerState _array_element))))

(fn ConstructionScript)

(fn DefineResources
  (bind _newresources (LocalVariables|GetNewResources))
  (bind _outrownames (DataTable|GetDataTableRowNames "/Game/UnrealDiplomacy/Data/DTUDResources.DTUDResources"))
  (for _array_element _outrownames
    (bind _returnvalue (Utilities|GetDataTableRow "/Game/UnrealDiplomacy/Data/DTUDResources.DTUDResources" _array_element)
      (:then
        (Utilities|Array|Add _newresources _returnvalue))))
  (return _newresources))

(fn GetPlayerData
  (params (JoinId :type Integer))
  (bind _playertoresources (Variables|Default|GetPlayerToResources))
  (if (Utilities|Array|IsValidIndex _playertoresources JoinId)
    ;[1 1 1] Return data
    (return (Utilities|Array|Get(acopy) _playertoresources JoinId))
    (else
      ;[1 1 1] Return fake
      (return (Utilities|Struct|MakeFUDPlayerData JoinId)))))

(fn CreatePlayerData
  (params (JoinId :type Integer))
  (bind _resources (CallFunction|DefineResources))
  (Utilities|Array|Add (Variables|Default|GetPlayerToResources) (Utilities|Struct|MakeFUDPlayerData JoinId "" "NewEnumerator1" "NewEnumerator0" _resources)))

(fn OnRepIsDirty
  (CallFunction|DisplayedDataChanged))