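; Simulation manager for the UnrealDiplomacy game that owns the player roster and the map manager.
; On BeginPlay it spawns a hex tile grid manager and keeps it as the local map.
; The world player is created first as the server-owned ID 0, clearing the roster, and later AI or human players take their array index as unique ID.
; Action processing is an empty stub.
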(event Custom|ProcessAction
  (params (ActionData :type FUD%20Action%20Data%20Structure)))

(event EventBeginPlay
  (CallFunction|CreateMapManager))

(event Collision|EventActorBeginOverlap
  (params (OtherActor :type Actor%20Object%20Reference)))

(event EventTick
  (params (DeltaSeconds :type Float%20%28single-precision%29)))

(fn ConstructionScript)

(fn CreateMapManager
  (bind _returnvalue (Game|SpawnActorfromClass "/Game/UnrealDiplomacy/Core/Managers/BP_AUDHexTileGridManager.BP_AUDHexTileGridManager_C" (Math|Conversions|ToTransform(Vector) "0, 0,20.000000") "Undefined" self 0))
  (Variables|Default|SetLocalMap _returnvalue)
  (return))

(fn CreateWorldPlayer
  (bind _players (Variables|Default|GetPlayers))
  ;[1 1 1] Creates a player that is owned by server, setting his unique to default value as it must always be first player that is created.
  (Utilities|Array|Clear _players)
  (bind _returnvalue (Utilities|Array|Add _players (Utilities|Struct|MakeFUDPlayer 0 "NewEnumerator0")))
  (return _returnvalue))

(fn CreatePlayer
  (params (Owner :type EUDPlayerOwner%20Enum :default "NewEnumerator0"))
  (bind _players (Variables|Default|GetPlayers))
  ;[1 1 1] Creates a player that is owned by either AI or Human, unique id is determined by current length of array. Returned index is same as we assign length and that directly transforms to same index due to 0 indexing.
  (bind _returnvalue (Utilities|Array|Add _players (Utilities|Struct|MakeFUDPlayer (Utilities|Array|Length _players) Owner)))
  (return _returnvalue))