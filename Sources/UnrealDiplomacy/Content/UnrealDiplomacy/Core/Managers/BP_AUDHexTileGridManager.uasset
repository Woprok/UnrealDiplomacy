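; Hex tile grid manager that stores lobby map settings and builds the world tile map.
; DefineMapParameters copies seed, minimum grid size, player radii and border thickness from lobby settings, using the larger of current and configured player counts.
; GenerateWorldTileMap nests height and width loops to return rows of identical placeholder tiles.
; Generation reads the usable grid dimensions, which are not computed here, and does not use the seed.
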(event EventBeginPlay)

(event Collision|EventActorBeginOverlap
  (params (OtherActor :type Actor%20Object%20Reference)))

(event EventTick
  (params (DeltaSeconds :type Float%20%28single-precision%29)))

(fn ConstructionScript)

(fn GenerateWorldTileMap
  (bind _newlocalvar_0 (LocalVariables|GetNewLocalVar_0))
  (for _index (range _newlocalvar_0 (Variables|Default|GetUseableGridHeight))
    (Utilities|Array|Clear (LocalVariables|GetNewRow))
    (for _index_2 (range _newlocalvar_0 (Variables|Default|GetUseableGridWidth))
      (Utilities|Array|Add (LocalVariables|GetNewRow) (Utilities|Struct|MakeUDTile (Utilities|Struct|MakeUDTileRegion "hal") (Utilities|Struct|MakeUDTileBiome "hal") (Utilities|Array|MakeArray (Utilities|Struct|MakeUDTileFeature "hal")))))
    (Utilities|Array|Add (Variables|Default|GetWorldTileRows) (Utilities|Struct|MakeUDTileRow (LocalVariables|GetNewRow))))
  (return (Variables|Default|GetWorldTileRows)))

(fn DefineMapParameters
  (params (LobbySettings :type FUD%20Lobby%20Settings%20Structure) (CurrentPlayerCount :type Integer))
  (bind (_mapseed _minimumwidth _minimumheight _playerexclusionradius _playerbufferradius _playercount _bordertilethickness) (Utilities|Struct|BreakFUDLobbySettings LobbySettings))
  (Utilities|FlowControl|Sequence
    (:then_0
      (if (> CurrentPlayerCount _playercount)
        (Variables|Default|SetPlayerCount CurrentPlayerCount)
        (else
          (Variables|Default|SetPlayerCount _playercount))))
    (:then_1
      (Variables|Default|SetMapSeed _mapseed))
    (:then_2
      (Variables|Default|SetMinimumGridWidth _minimumwidth))
    (:then_3
      (Variables|Default|SetMinimumGridHeight _minimumheight))
    (:then_4
      (Variables|Default|SetPlayerExclusionRadius _playerexclusionradius))
    (:then_5
      (Variables|Default|SetPlayerBufferRadius _playerbufferradius))
    (:then_6
      (Variables|Default|SetBorderTileThickness _bordertilethickness))
    (:then_7
      (return))))