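; Hex grid manager that generates the seeded world tile map for a diplomacy game from lobby settings and a player list.
; It builds a tile table and unused-position pool, then gives each player a random capital matching their nation.
; Recursive neighbor expansion, using odd/even row offsets, fills a nation-biased exclusion zone and a random buffer around each capital.
; Leftover positions get random region, biome and features from cached data tables.
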(event EventBeginPlay)

(event Collision|EventActorBeginOverlap
  (params (OtherActor :type Actor%20Object%20Reference)))

(event EventTick
  (params (DeltaSeconds :type Float%20%28single-precision%29)))

(fn ConstructionScript)

(fn GenerateWorldTileMap
  (params (Players :type Array%20of%20FUD%20Player%20Data%20Structures))
  (bind _udtile (Generation|CreateRandomTile))
  (bind (_owner _region _biome _features) (Utilities|Struct|BreakUDTile _udtile))
  (Utilities|FlowControl|Sequence
    (:then_0
      ;[1 1 1] Initialize tables used in generation and result table
      (Utilities|CreateRandomizationArrays
        (:Completed
          (Utilities|CreateTileTable
            (:Completed
              (Utilities|InitRandomCache))))))
    (:then_1
      ;[1 1 1] For each player determine spawn position
      (for _array_element Players
        (bind _structout (Utilities|Struct|SetmembersinFUDPlayerData _array_element (Helper|TakeRandomUnusedPosition)))
        (Generation|UpdateSpawnandSurrounding (.UniqueId (Utilities|Struct|BreakFUDPlayerData _structout)) (.Nation (Utilities|Struct|BreakFUDPlayerData _structout)) (.StartPosition (Utilities|Struct|BreakFUDPlayerData _structout)))))
    (:then_2
      ;[1 1 1] Remaining tiles are assigned randomly as well
      (for _array_element_2 (Variables|Generation|GetRandomizationArray)
        (Utilities|Struct|SetmembersinUDTile (Utilities|GetTileReference (.X (Utilities|Struct|BreakIntPoint _array_element_2)) (.Y (Utilities|Struct|BreakIntPoint _array_element_2))) _region _biome _features))
      (return (Variables|Default|GetTileTable)))))

(fn DefineMapParameters
  (params (LobbySettings :type FUD%20Lobby%20Settings%20Structure) (CurrentPlayerCount :type Integer))
  (bind (_mapseed _minimumwidth _minimumheight _playerexclusionradius _playerbufferradius _playercount _bordertilethickness) (Utilities|Struct|BreakFUDLobbySettings LobbySettings))
  (Utilities|FlowControl|Sequence
    (:then_0
      (if (> CurrentPlayerCount _playercount)
        (Variables|Default|SetPlayerCount CurrentPlayerCount)
        (else
          (Variables|Default|SetPlayerCount _playercount))))
    (:then_1
      (Variables|Default|SetMapSeed _mapseed))
    (:then_2
      (Variables|Default|SetMinimumGridWidth _minimumwidth))
    (:then_3
      (Variables|Default|SetMinimumGridHeight _minimumheight))
    (:then_4
      (Variables|Default|SetPlayerExclusionRadius _playerexclusionradius))
    (:then_5
      (Variables|Default|SetPlayerBufferRadius _playerbufferradius))
    (:then_6
      (Variables|Default|SetBorderTileThickness _bordertilethickness))
    (:then_7
      (return))))

(fn IsOddRow
  (params (A :type Integer))
  (return (== (Math|Integer|%(Integer) A 2) 1)))

(fn TakeSurroundingUnusedPositions
  (params (X :type Integer) (Y :type Integer))
  (bind _intpoint (Utilities|Struct|MakeIntPoint X Y))
  ;[1 1 1] We need to get all possible sides, in our case we use hexes == 6, we will also use remove action so randomization array is after this smaller
  (Utilities|FlowControl|Sequence
    (:then_0
      (Utilities|Array|Clear (LocalVariables|GetUnusedSurrounds))
      (if (Helper|IsOddRow X)
        (for _array_element (LocalVariables|GetOddSurroundingTilesIndices)
          (bind _position (Utilities|TakeUnusedPosition (+ _array_element _intpoint))
            (:Found
              (Utilities|Array|Add (LocalVariables|GetUnusedSurrounds) _position))))
        (else
          (for _array_element_2 (LocalVariables|GetEvenSurroundingTilesIndices)
            (bind _position_2 (Utilities|TakeUnusedPosition (+ _array_element_2 _intpoint))
              (:Found
                (Utilities|Array|Add (LocalVariables|GetUnusedSurrounds) _position_2)))))))
    (:then_1
      (return (LocalVariables|GetUnusedSurrounds)))))

(fn TakeRandomUnusedPosition
  (bind _randomstream (Variables|Generation|GetRandomStream))
  (bind _randomizationarray (Variables|Generation|GetRandomizationArray))
  (bind _returnvalue (Utilities|Array|Length _randomizationarray))
  (bind _returnvalue_2 (Class|KismetMathLibrary|RandomIntegerfromStream _returnvalue _randomstream))
  (Utilities|Array|RemoveIndex _randomizationarray _returnvalue_2)
  (return (Utilities|Array|Get(acopy) _randomizationarray _returnvalue_2)))

(fn GetRandomRegion
  (return (.OutItem (Utilities|Array|RandomFromStream (Variables|RandomizationCache|GetCachedRegions) (Variables|Generation|GetRandomStream)))))

(fn GerRandomBiome
  (return (.OutItem (Utilities|Array|RandomFromStream (Variables|RandomizationCache|GetCachedBiomes) (Variables|Generation|GetRandomStream)))))

(fn GetRandomFeatures
  (params (StartFeature :type UD%20Tile%20Feature%20Structure) (HasStartFeature :type Boolean) (DoMax :type Boolean))
  (bind _maxtilefeatures (Variables|Generation|GetMaxTileFeatures))
  (bind _randomstream (Variables|Generation|GetRandomStream))
  (bind _newfeatures (LocalVariables|GetNewFeatures))
  (Utilities|Array|Clear _newfeatures)
  (if HasStartFeature
    (Utilities|Array|Add _newfeatures StartFeature))
  (if DoMax
    ;[1 1 1] Max is in both branches same as true branch is < false one is <= resulting in the same 0,1,2 for 3 and 0,1,2 for random 3, which is max 2
    (Utilities|StandardforLoop 0 _maxtilefeatures
      (:LoopBody
        (Utilities|Array|Add (LocalVariables|GetNewFeatures) (.OutItem (Utilities|Array|RandomFromStream (Variables|RandomizationCache|GetCachedFeatures) _randomstream)) :!label _label))
      (:Completed
        (return (LocalVariables|GetNewFeatures))))
    (else
      (for _index (range 0 (Class|KismetMathLibrary|RandomIntegerfromStream _maxtilefeatures _randomstream))
        (goto _label))
      (return (LocalVariables|GetNewFeatures)))))

(fn UpdateSpawnandSurrounding
  (params (OwnerId :type Integer) (Nation :type FUD%20Nation%20Settings%20Structure%20%28by%20ref%29) (Position :type Int%20Point%20Structure%20%28by%20ref%29))
  (bind (_x _y) (Utilities|Struct|BreakIntPoint Position))
  (bind (_region _biome _feature) (Utilities|Struct|BreakFUDNationSettings Nation))
  (Utilities|FlowControl|Sequence
    (:then_0
      ;[1 1 1] Spawn Capital Tile
      (Utilities|Struct|SetmembersinUDTile (Utilities|GetTileReference _x _y) OwnerId _region _biome (Generation|GetRandomFeatures _feature true true)))
    (:then_1
      ;[1 1 1] Generate Surroundings
      (Generation|RecursiveSurroundingCreation _x _y (Variables|Default|GetPlayerExclusionRadius) (Variables|Default|GetPlayerBufferRadius) Nation))
    (:then_2
      (return))))

(fn CreateRandomNationTile
  (params (NationPreference :type FUD%20Nation%20Settings%20Structure))
  (bind (_region _biome _feature) (Utilities|Struct|BreakFUDNationSettings NationPreference))
  (bind _region_2 (Generation|GetRandomRegion))
  (bind _features (Generation|GetRandomFeatures))
  (bind _biome_2 (Generation|GerRandomBiome))
  (switch int (Class|KismetMathLibrary|RandomIntegerfromStream 3 (Variables|Generation|GetRandomStream))
    (:0
      (return (Utilities|Struct|MakeUDTile 0 _region _biome_2 _features)))
    (:1
      (return (Utilities|Struct|MakeUDTile 0 _region_2 _biome _features)))
    (:2
      (return (Utilities|Struct|MakeUDTile 0 _region_2 _biome_2 (Generation|GetRandomFeatures _feature true false))))))

(fn CreateRandomTile
  ;[1 1 1] Random using default randomization effort, without additional bonus
  (return (Utilities|Struct|MakeUDTile 0 (Generation|GetRandomRegion) (Generation|GerRandomBiome) (Generation|GetRandomFeatures))))

(fn RecursiveSurroundingCreation
  (params (X :type Integer) (Y :type Integer) (RemainingExclusion :type Integer) (RemainingBuffer :type Integer) (NationPreference :type FUD%20Nation%20Settings%20Structure))
  (bind _udtile (Generation|CreateRandomNationTile NationPreference))
  (bind _udtile_2 (Generation|CreateRandomTile))
  (bind (_owner _region _biome _features) (Utilities|Struct|BreakUDTile _udtile))
  (bind (_owner_2 _region_2 _biome_2 _features_2) (Utilities|Struct|BreakUDTile _udtile_2))
  ;[1 1 1] Supplied tile must be solved, we are solving ony surronding
  (bind _output_get (LocalVariables|SetTempSurroundings (Helper|TakeSurroundingUnusedPositions X Y)))
  ;[1 1 1] Are we in exclusion, or are we moving to buffer ?
  (if (> RemainingExclusion 0)
    ;[1 1 1] Solve current level and then move to next level using recursion.
    (for _array_element _output_get
      (Utilities|Struct|SetmembersinUDTile (Utilities|GetTileReference (.X (Utilities|Struct|BreakIntPoint _array_element)) (.Y (Utilities|Struct|BreakIntPoint _array_element))) _region _biome _features))
    (for _array_element_2 _output_get
      (Generation|RecursiveSurroundingCreation (.X (Utilities|Struct|BreakIntPoint _array_element_2)) (.Y (Utilities|Struct|BreakIntPoint _array_element_2)) (- RemainingExclusion 1) RemainingBuffer NationPreference))
    (else
      ;[1 1 1] Are we in buffer, or are we at the end ?
      (if (> RemainingBuffer 0)
        ;[1 1 1] This resolves buffer, potentially it will interfere with exclusion nation preference, but thats acceptable as we are not going to care about little imbalances in map gen. Might be reworked with extending how is it calculated or forcing buffer to be used after exclusion only by creating strict exclusion to buffer
        (for _array_element_3 _output_get
          (Utilities|Struct|SetmembersinUDTile (Utilities|GetTileReference (.X (Utilities|Struct|BreakIntPoint _array_element_3)) (.Y (Utilities|Struct|BreakIntPoint _array_element_3))) _region_2 _biome_2 _features_2))
        (for _array_element_4 _output_get
          (Generation|RecursiveSurroundingCreation (.X (Utilities|Struct|BreakIntPoint _array_element_4)) (.Y (Utilities|Struct|BreakIntPoint _array_element_4)) -1 (- RemainingBuffer 1) NationPreference))
        (else
          ;[1 1 1] Finished this recursion level
          (return))))))