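; BP_AUDHexTile is a clickable hex map tile actor with selected and unselected border materials.
; RefreshVisuals flips the replicated VisualChangeTag, whose RepNotify calls VisualUpdate as a change signal, while UpdateVisuals passes tile data to VisualUpdateFrom.
; Both visual update functions are empty here.
; Clicks on WORLD tiles only fetch the player controller, with no further action wired.
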(event Custom|OnSelected
  (Rendering|Material|SetMaterial (Variables|Default|GetBorder) 0 "/Game/UnrealDiplomacy/Development/HexTiles/MI_HexTile_BackgroundSelected.MI_HexTile_BackgroundSelected"))

(event Custom|OnDeselected
  (Rendering|Material|SetMaterial (Variables|Default|GetBorder) 0 "/Game/UnrealDiplomacy/Development/HexTiles/MI_HexTile_BackgroundUnselected.MI_HexTile_BackgroundUnselected"))

(event Custom|RefreshVisuals
  (Utilities|UpdateVisualChangeTag))

(event Custom|UpdateVisuals
  (params (TileData :type UD%20Tile%20Structure))
  (CallFunction|VisualUpdatefrom TileData))

(event Custom|OnClicked_Event
  (params (TouchedActor :type Actor%20Object%20Reference) (ButtonPressed :type Key%20Structure :default "None")))

(event EventBeginPlay)

(event MouseInput|EventActorOnClicked
  (params (ButtonPressed :type Key%20Structure :default "None"))
  (switch Utilities|FlowControl|Switch|SwitchonEHexTileType (Variables|Default|GetTileType)
    (:WORLD
      (CallFunction|GetUDPlayerController))))

(fn ConstructionScript)

(fn OnRepVisualChangeTag
  (CallFunction|VisualUpdate)
  (return))

(fn VisualUpdate
  (return))

(fn VisualUpdatefrom
  (params (TileData :type UD%20Tile%20Structure))
  (return))