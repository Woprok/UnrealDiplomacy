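; Blueprint world hex tile for UnrealDiplomacy that shows each tile's biome and realm on the map.
; VisualUpdateFrom picks the tile mesh material from the biome name, then calls the parent; VisualUpdate runs it with no tile data wired.
; OnVisualUpdate lowers Deepcrust Realm tiles and raises Cloudcrust Realm tiles relative to their current height, so repeated events accumulate.
; It also logs the tile's position and biome.
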(event EventOnVisualUpdate
  (params (tile :type UD%20Tile%20Structure%20%28by%20ref%29))
  (bind (_owner _worldposition _region _biome) (Utilities|Struct|BreakUDTile tile))
  (bind _rootcomponent (Variables|Transformation|GetRootComponent))
  (bind _rootcomponent_2 (Variables|Transformation|GetRootComponent))
  (bind _returnvalue (Transformation|GetWorldLocation _rootcomponent))
  (bind _returnvalue_2 (Transformation|GetWorldLocation _rootcomponent_2))
  (switch string (Utilities|Struct|BreakUDTileRegion _region)
    (:Deepcrust%20Realm
      (Transformation|SetWorldLocation _rootcomponent (Math|Vector|MakeVector (.x _returnvalue) (.y _returnvalue) (- (.z _returnvalue) 25.0)) false true))
    (:Realm
      _)
    (:Cloudcrust%20Realm
      (Transformation|SetWorldLocation _rootcomponent_2 (Math|Vector|MakeVector (.x _returnvalue_2) (.y _returnvalue_2) (+ (.z _returnvalue_2) 25.0)) false true)))
  (CallFunction|LogInfo (Utilities|String|Append (Utilities|String|ToString(Integer) _worldposition) " - " (Utilities|Struct|BreakUDTileBiome _biome)) false))

(fn ConstructionScript
  (|CallParentFunction))

(fn VisualUpdate
  (bind _asbp_udplayer_controller (CallFunction|GetUDPlayerController))
  (CallFunction|GetUDGameState)
  (Utilities|FlowControl|Sequence
    (:then_0
      (CallFunction|VisualUpdatefrom))
    (:then_1
      (|CallParentFunction)
      (return))))

(fn VisualUpdatefrom
  (params (TileData :type UD%20Tile%20Structure))
  (Utilities|FlowControl|Sequence
    (:then_0
      (switch string (Utilities|Struct|BreakUDTileBiome (.Biome (Utilities|Struct|BreakUDTile TileData)))
        (:Desert
          (Rendering|Material|SetMaterial (Variables|Default|GetTileMesh) 0 "/Game/UnrealDiplomacy/Development/HexTiles/MI_HexTile_BiomeDesert.MI_HexTile_BiomeDesert"))
        (:Savanna
          (Rendering|Material|SetMaterial (Variables|Default|GetTileMesh) 0 "/Game/UnrealDiplomacy/Development/HexTiles/MI_HexTile_BiomeSavanna.MI_HexTile_BiomeSavanna"))
        (:Temperate
          (Rendering|Material|SetMaterial (Variables|Default|GetTileMesh) 0 "/Game/UnrealDiplomacy/Development/HexTiles/MI_HexTile_BiomeTemperate.MI_HexTile_BiomeTemperate"))
        (:Steppe
          (Rendering|Material|SetMaterial (Variables|Default|GetTileMesh) 0 "/Game/UnrealDiplomacy/Development/HexTiles/MI_HexTile_BiomeSteppe.MI_HexTile_BiomeSteppe"))
        (:Tropical
          (Rendering|Material|SetMaterial (Variables|Default|GetTileMesh) 0 "/Game/UnrealDiplomacy/Development/HexTiles/MI_HexTile_BiomeTropical.MI_HexTile_BiomeTropical"))
        (:Tundra
          (Rendering|Material|SetMaterial (Variables|Default|GetTileMesh) 0 "/Game/UnrealDiplomacy/Development/HexTiles/MI_HexTile_BiomeTundra.MI_HexTile_BiomeTundra"))
        (:Alpine
          (Rendering|Material|SetMaterial (Variables|Default|GetTileMesh) 0 "/Game/UnrealDiplomacy/Development/HexTiles/MI_HexTile_BiomeAlpine.MI_HexTile_BiomeAlpine"))
        (:Arctic
          (Rendering|Material|SetMaterial (Variables|Default|GetTileMesh) 0 "/Game/UnrealDiplomacy/Development/HexTiles/MI_HexTile_BiomeArctic.MI_HexTile_BiomeArctic"))))
    (:then_1
      (|CallParentFunction TileData)
      (return))))